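; Placeable housing plot that offers a house for purchase, removing itself on load if the game instance's housing map matches its own.
; A child BP_InteractionActor, shaped and positioned in the construction script along with the mesh and info text, drives an affordability-colored custom-depth outline and the interaction.
; Interacting freezes movement and opens the BP_HousingBuy widget in UI-only input.
; ExitHousingBuy restores control and destroys the plot.
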(event `self.ReceiveBeginPlay`
  (bind _interactionactor (`self.InteractionActor`))
  (`/Game/LS_Template/Blueprints/Interaction/Core/BP_InteractionActor.SetWidget` _interactionactor (`self.HouseName`) false 0 0)
  (add `/Game/LS_Template/Blueprints/Interaction/Core/BP_InteractionActor.OnSetUseable` _interactionactor (delegate `OnSetUseable`))
  (add `/Game/LS_Template/Blueprints/Interaction/Core/BP_InteractionActor.OnSetUnuseable` _interactionactor (delegate `OnSetUnuseable`))
  (add `/Game/LS_Template/Blueprints/Interaction/Core/BP_InteractionActor.OnInteraction` _interactionactor (delegate `OnInteraction`))
  ;[1 1 1] Delay for loading purposes
  (`KismetSystemLibrary.Delay` 0.1)
  ;[1 1 1] Destroys the actor if the house has already been bought
  (if (`KismetStringLibrary.EqualEqual_StrStr` (`/Game/LS_Template/Blueprints/Systems/Core/LS_Instance.HousingMapName` (`/Game/LS_Template/Blueprints/Systems/Core/BPL_Functions.Get_LST_Instance`)) (`self.HousingMapName`))
    (`self.K2_DestroyActor`)))

(event `OnSetUseable`
  (`self.SetMeshOutline` true))

(event `OnSetUnuseable`
  (`self.SetMeshOutline` false))

(event `OnInteraction`
  (`self.HousingPlotInteraction`))

(event `HousingPlotInteraction`
  (bind _w_playerhud (`/Game/LS_Template/Blueprints/Systems/Core/BPL_Functions.Get_LST_PlayerHUD`))
  (bind _lst_controller (`/Game/LS_Template/Blueprints/Systems/Core/BPL_Functions.Get_LST_Controller`))
  ;[1 1 1] Is the HUD visible ? If false, then hide it
  (if (`/Game/LS_Template/Blueprints/UI/W_PlayerHUD.IsInventoryVisible` _w_playerhud)
    (`/Game/LS_Template/Blueprints/UI/W_PlayerHUD.DisplayHUD` _w_playerhud false true))
  ;[1 1 1] Disable movement during interactions
  (`CharacterMovementComponent.DisableMovement` (`Character.CharacterMovement` (`GameplayStatics.GetPlayerCharacter` 0)))
  (bind _returnvalue (`|CreateWidget` "/Game/LS_Template/Blueprints/Housing/BP_HousingBuy.BP_HousingBuy_C" null (`self.HouseName`) (`self.HousePrice`) self))
  (bind _output_get (set `self.W_HousingBuy` _returnvalue))
  (`UserWidget.AddToViewport` _output_get 0)
  (set `PlayerController.bShowMouseCursor` true _lst_controller)
  (`WidgetBlueprintLibrary.SetInputMode_UIOnlyEx` _lst_controller (`self.W_HousingBuy`)))

(event `ExitHousingBuy`
  (bind _lst_controller (`/Game/LS_Template/Blueprints/Systems/Core/BPL_Functions.Get_LST_Controller`))
  (`CharacterMovementComponent.SetMovementMode` (`Character.CharacterMovement` (`GameplayStatics.GetPlayerCharacter` 0)) "MOVE_Walking" 0)
  (set `PlayerController.bShowMouseCursor` false _lst_controller)
  (`WidgetBlueprintLibrary.SetInputMode_GameOnly` _lst_controller)
  (`self.K2_DestroyActor`))

(fn `SetMeshOutline`
  (params (`Outline?` :type Boolean))
  (if (`/Game/LS_Template/Blueprints/Systems/Core/LS_Instance.UseMeshOutline?` (`/Game/LS_Template/Blueprints/Systems/Core/BPL_Functions.Get_LST_Instance`))
    (`MaterialInstanceDynamic.SetVectorParameterValue` (`/Game/LS_Template/Blueprints/Interaction/Core/BPC_Interaction.OutlineDynamat` (`/Game/LS_Template/Blueprints/Systems/Core/Game/BP_LS_GameController.BPC_Interaction` (`/Game/LS_Template/Blueprints/Systems/Core/BPL_Functions.Get_LST_Controller`))) "OutlineColor" (select `bool` (>= (`/Game/LS_Template/Blueprints/Systems/Core/BPL_Functions.GetCurrentMoney`) (`self.HousePrice`)) :`false` (struct :`R` 0.901042 :`G` 0.092801 :`B` 0.074874 :`A` 1.0) :`true` (struct :`R` 0.241749 :`G` 0.921875 :`B` 0.187397 :`A` 1.0) :!type "LinearColor Structure"))
    (`PrimitiveComponent.SetRenderCustomDepth` (`self.SM_HousingPlot`) `Outline?`)
    (return)
    (else
      (return))))

(fn `UserConstructionScript`
  (bind _sm_housingplot (`self.SM_HousingPlot`))
  (bind _asbp_interaction_actor (cast `/Game/LS_Template/Blueprints/Interaction/Core/BP_InteractionActor` (`ChildActorComponent.ChildActor` (`self.ChildActor`))))
  (bind _output_get (set `self.InteractionActor` _asbp_interaction_actor))
  (`/Game/LS_Template/Blueprints/Interaction/Core/BP_InteractionActor.HandleInteractionShape` _output_get (`self.InteractionShape`) (`self.SphereRadius`) (`self.BoxExtent`) (`self.CapsuleHalfHeight`) (`self.CapsuleRadius`))
  (`self.K2_SetActorRelativeLocation` _output_get (`self.InteractionLocation`) false false)
  (`SceneComponent.K2_SetRelativeLocation` (`/Game/LS_Template/Blueprints/Interaction/Core/BP_InteractionActor.Widget` _output_get) (`self.PromptLocation`) false false)
  (`StaticMeshComponent.SetStaticMesh` _sm_housingplot (`self.HousingPlotMesh`))
  (`SceneComponent.SetRelativeScale3D` _sm_housingplot (`self.HousingPlotMeshScale`))
  (`TextRenderComponent.K2_SetText` (`self.TextRender`) (`|FormatText` "House Name : {HouseName} \nPrice : {Price} credits \nMap : {HousingMapName}" (`self.HouseName`) (`KismetTextLibrary.Conv_IntToText` (`self.HousePrice`)) (`KismetTextLibrary.Conv_StringToText` (`self.HousingMapName`)))))