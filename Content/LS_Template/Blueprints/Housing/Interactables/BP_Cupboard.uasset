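; BP_Cupboard is an interactable housing cupboard that opens a cupboard UI when used.
; On InteractionEvent it calls DisplayHUD on the LST player HUD if the inventory is visible, then shows a W_Cupboard widget, created on first use and cached for reuse.
; It then switches the LST controller to UI-only input focused on that widget and shows the mouse cursor.
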(event `self.InteractionEvent`
  (bind _w_playerhud (`/Game/LS_Template/Blueprints/Systems/Core/BPL_Functions.Get_LST_PlayerHUD`))
  (bind _lst_controller (`/Game/LS_Template/Blueprints/Systems/Core/BPL_Functions.Get_LST_Controller`))
  (if (`/Game/LS_Template/Blueprints/UI/W_PlayerHUD.IsInventoryVisible` _w_playerhud)
    (`/Game/LS_Template/Blueprints/UI/W_PlayerHUD.DisplayHUD` _w_playerhud false true))
  (`/Engine/EditorBlueprintResources/StandardMacros.IsValid` (`self.W_Cupboard`)
    (:`Is Valid`
      _)
    (:`Is Not Valid`
      (bind _returnvalue (`|CreateWidget` "/Game/LS_Template/Blueprints/UI/Cupboard/W_Cupboard.W_Cupboard_C"))
      (set `self.W_Cupboard` _returnvalue)))
  (`UserWidget.AddToViewport` (`self.W_Cupboard`) -1)
  (`WidgetBlueprintLibrary.SetInputMode_UIOnlyEx` _lst_controller (`self.W_Cupboard`))
  (set `PlayerController.bShowMouseCursor` true _lst_controller))

(fn `UserConstructionScript`
  (`parent.UserConstructionScript`))