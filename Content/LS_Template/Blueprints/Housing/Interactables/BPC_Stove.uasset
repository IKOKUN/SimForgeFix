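; Interactable housing stove that opens a crafting menu for the player.
; Interacting shows the player HUD's inventory if it is hidden, then adds a crafting widget in non-workbench mode to the viewport.
; The widget is created on first use and cached for later interactions.
; When an actor instigated by the player's controller ends overlap, the menu closes if it is on screen.
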(event `self.InteractionEvent`
  (bind _w_playerhud (`/Game/LS_Template/Blueprints/Systems/Core/BPL_Functions.Get_LST_PlayerHUD`))
  (if (not (`/Game/LS_Template/Blueprints/UI/W_PlayerHUD.IsInventoryVisible` _w_playerhud))
    (`/Game/LS_Template/Blueprints/UI/W_PlayerHUD.DisplayHUD` _w_playerhud false true))
  (`/Engine/EditorBlueprintResources/StandardMacros.IsValid` (`self.W_CraftingMenu`)
    (:`Is Valid`
      _)
    (:`Is Not Valid`
      (bind _returnvalue (`|CreateWidget` "/Game/LS_Template/Blueprints/UI/Crafting/W_CraftingMenu.W_CraftingMenu_C"))
      (set `self.W_CraftingMenu` _returnvalue)))
  (`UserWidget.AddToViewport` (`self.W_CraftingMenu`) -1))

(event `self.OnEndOverlap`
  (params (OverlappedActor :type "Actor Object Reference") (OtherActor :type "Actor Object Reference"))
  (bind _w_craftingmenu (`self.W_CraftingMenu`))
  (`/Engine/EditorBlueprintResources/StandardMacros.IsValid` (`self.W_CraftingMenu`)
    (:`Is Valid`
      (if (and (== (`self.GetInstigatorController` OtherActor) (`/Game/LS_Template/Blueprints/Systems/Core/BPL_Functions.Get_LST_Controller`)) (and (`Widget.IsInViewport` _w_craftingmenu) (`KismetSystemLibrary.IsValid` _w_craftingmenu)))
        (`/Game/LS_Template/Blueprints/UI/Crafting/W_CraftingMenu.OnMenuClose` (`self.W_CraftingMenu`))))))

(fn `UserConstructionScript`
  (`parent.UserConstructionScript`))