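; Housing interactable radio that the player switches on and off to play music.
; The interaction event flip-flops between playing and stopping a music cue attached to the housing mesh.
; The sound component is spawned on demand when no valid one exists, and playback always starts from the beginning.
; Each toggle updates the Switch On/Off prompt text through InteractionActor, then calls HidePrompt on it.
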(event `self.ReceiveBeginPlay`
  (`parent.ReceiveBeginPlay`)
  (`/Game/LS_Template/Blueprints/Interaction/Core/BP_InteractionActor.SetWidget` (`self.InteractionActor`) "Radio : Switch On" false 0 0))

(event `self.InteractionEvent`
  (bind _playedsound (`self.PlayedSound`))
  (bind _interactionactor (`self.InteractionActor`))
  (bind _isa (`/Engine/EditorBlueprintResources/StandardMacros.FlipFlop`)
    (:`A`
      (`/Engine/EditorBlueprintResources/StandardMacros.IsValid` _playedsound
        (:`Is Valid`
          _)
        (:`Is Not Valid`
          (bind _returnvalue (`GameplayStatics.SpawnSoundAttached` "/Game/LS_Template/EpicContent/StarterContent/Audio/Starter_Music_Cue.Starter_Music_Cue" (`self.SM_HousingMesh`) "None" (0.0 0.0 0.0) (struct) "KeepRelativeOffset" false 1.0 1.0 0.0 null null))
          (set `self.PlayedSound` _returnvalue)))
      (`AudioComponent.Play` _playedsound 0.0))
    (:`B`
      (`AudioComponent.Stop` (`self.PlayedSound`))))
  (`/Game/LS_Template/Blueprints/Interaction/Core/BP_InteractionActor.SetWidget` _interactionactor (select `bool` _isa :`false` "Radio : Switch On" :`true` "Radio : Switch Off" :!type "Text") false 0 0)
  (`/Game/LS_Template/Blueprints/Interaction/Core/BP_InteractionActor.HidePrompt` _interactionactor true))

(fn `UserConstructionScript`
  (`parent.UserConstructionScript`))