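; BPC_Bed is an interactable housing bed that lets the player sleep to jump to a set time of day.
; BeginPlay sets the interaction widget text to "Sleep".
; On interaction, it disables input on the LST controller and player character, fades out camera and audio, advances to a fixed daytime, fades back in, then restores input, using delays to match each fade.
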(event `self.ReceiveBeginPlay`
  (`parent.ReceiveBeginPlay`)
  (`/Game/LS_Template/Blueprints/Interaction/Core/BP_InteractionActor.SetWidget` (`self.InteractionActor`) "Sleep" false 0 0))

(event `self.InteractionEvent`
  (bind _lst_controller (`/Game/LS_Template/Blueprints/Systems/Core/BPL_Functions.Get_LST_Controller`))
  (bind _lst_controller_2 (`/Game/LS_Template/Blueprints/Systems/Core/BPL_Functions.Get_LST_Controller`))
  (`self.DisableInput` _lst_controller_2 _lst_controller_2)
  (`self.DisableInput` (`GameplayStatics.GetPlayerCharacter` 0) _lst_controller_2)
  (`/Game/LS_Template/Blueprints/Systems/Core/BPL_Functions.CameraFadeOut` 2.0 true)
  (`KismetSystemLibrary.Delay` 2.0)
  (`/Game/LS_Template/Blueprints/Systems/Core/BPL_Functions.AdvanceDayTime` true "NewEnumerator1")
  (`/Game/LS_Template/Blueprints/Systems/Core/BPL_Functions.CameraFadeIn` 2.0)
  (`KismetSystemLibrary.Delay` 2.0)
  (`self.EnableInput` _lst_controller _lst_controller)
  (`self.EnableInput` (`GameplayStatics.GetPlayerCharacter` 0) _lst_controller))

(fn `UserConstructionScript`
  (`parent.UserConstructionScript`))