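; BP_Painting is an interactable housing furniture painting that switches between two colors when used.
; On BeginPlay it creates a dynamic material instance from the SMFurniture mesh's first material and applies it back to that slot.
; Each InteractionEvent uses a FlipFlop to set the material's Color parameter to green or red, then shows the interaction prompt again through the interactor.
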(event `self.ReceiveBeginPlay`
  (`parent.ReceiveBeginPlay`)
  ;[1 1 1] Get the material of the mesh, create a dynamic instance and sets it to the mesh
  (bind _returnvalue (`KismetMaterialLibrary.CreateDynamicMaterialInstance` (`PrimitiveComponent.GetMaterial` (`self.SM_Furniture`) 0)))
  (bind _output_get (set `self.PaintingDynamat` _returnvalue))
  (`PrimitiveComponent.SetMaterial` (`self.SM_Furniture`) 0 _output_get))

(event `self.InteractionEvent`
  ;[1 1 1] Switch between two colors and show the item prompt after interaction
  (`/Engine/EditorBlueprintResources/StandardMacros.FlipFlop`
    (:`A`
      (`MaterialInstanceDynamic.SetVectorParameterValue` (`self.PaintingDynamat`) "Color" (struct :`R` 0.124779 :`G` 0.921875 :`B` 0.140728 :`A` 1.0)))
    (:`B`
      (`MaterialInstanceDynamic.SetVectorParameterValue` (`self.PaintingDynamat`) "Color" (struct :`R` 0.921875 :`G` 0.086205 :`B` 0.104547 :`A` 1.0))))
  (`/Game/LS_Template/Blueprints/Interaction/Core/BP_InteractionActor.HidePrompt` (`self.Interactor Actor`) false))

(fn `UserConstructionScript`
  (`parent.UserConstructionScript`))