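; Base actor for a placeable housing item, showing the mesh from its ItemInfo and becoming the controller's selection when clicked.
; On BeginPlay it replaces itself with the item's HousingClass if different, otherwise interactable items attach an interaction actor with outline and child-overridable events.
; While ticking it follows the cursor, grid-snapped with Left Shift.
; Wall items align yaw to non-horizontal surfaces; others use a downward trace.
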(event `self.ReceiveBeginPlay`
  (bind _interactionactor (`self.InteractionActor`))
  (bind (_iteminfo_itemrowname _iteminfo_itemname _iteminfo_itemdescription _iteminfo_itemtype _iteminfo_clothestype _iteminfo_itemrarity _iteminfo_itemicon _iteminfo_itemsound _iteminfo_simulatephysics_ _iteminfo_itemmesh _iteminfo_itemprice _iteminfo_itemamount _iteminfo_gaindetails _iteminfo_housingdetails) (break `/Game/LS_Template/Blueprints/Systems/Structures/Items/S_ItemInfo` (`self.ItemInfo`)))
  (bind (_wallitem_ _housinginteractable_ _housingclass) (break `/Game/LS_Template/Blueprints/Systems/Structures/Housing/S_HousingDetails` _iteminfo_housingdetails))
  ;[1 1 1] If the specified class is different in DT_Items, spawn the specified class and destroy this actor. This is used only for interactable housing items
  (if (!= _housingclass (`GameplayStatics.GetObjectClass` self))
    (`|SpawnActorFromClass` _housingclass (`self.GetTransform`) "AlwaysSpawn" "SelectDefaultAtRuntime" null (`self.ItemInfo`) (`self.HousingIndex`) (`self.MeshRotation`) (`self.MeshLocation`) null)
    (`self.K2_DestroyActor`)
    (else
      ;[1 1 1] If the housing item is interactable, spawns and attach an interaction actor
      (if _housinginteractable_
        (bind _returnvalue (`|SpawnActorFromClass` "/Game/LS_Template/Blueprints/Interaction/Core/BP_InteractionActor.BP_InteractionActor_C" (`KismetMathLibrary.MakeTransform` (`PrimitiveComponent.GetCenterOfMass` (`self.SM_HousingMesh`) "None")) "Undefined" "OverrideRootScale" null "NewEnumerator0" null))
        (bind _output_get (set `self.InteractionActor` _returnvalue))
        (`self.K2_AttachToComponent` _output_get (`self.SM_HousingMesh`) "None" "SnapToTarget" "SnapToTarget" "SnapToTarget" true)
        (add `/Game/LS_Template/Blueprints/Interaction/Core/BP_InteractionActor.OnSetUseable` _interactionactor (delegate `OnSetUseable`))
        (add `/Game/LS_Template/Blueprints/Interaction/Core/BP_InteractionActor.OnSetUnuseable` _interactionactor (delegate `OnSetUnuseable`))
        (add `/Game/LS_Template/Blueprints/Interaction/Core/BP_InteractionActor.OnInteraction` _interactionactor (delegate `InteractionEvent`))
        (add `self.OnActorBeginOverlap` _interactionactor (delegate `OnBeginOverlap`))
        (add `self.OnActorEndOverlap` _interactionactor (delegate `OnEndOverlap`))
        (`self.SetInteractionDefaults`)))))

(event `OnSetUseable`
  ;[1 1 1] If the housing item is interactable, spawns and attach an interaction actor
  (`self.SetOutline?` true))

(event `OnSetUnuseable`
  ;[1 1 1] If the housing item is interactable, spawns and attach an interaction actor
  (`self.SetOutline?` false))

(event `OnBeginOverlap` :!signature `self.OnActorBeginOverlap`
  (params (OverlappedActor :type "Actor Object Reference") (OtherActor :type "Actor Object Reference"))
  ;[1 1 1] If the housing item is interactable, spawns and attach an interaction actor
  ;;[1 1 1] Overriden in child blueprint
)

(event `OnEndOverlap` :!signature `self.OnActorEndOverlap`
  (params (OverlappedActor :type "Actor Object Reference") (OtherActor :type "Actor Object Reference"))
  ;[1 1 1] If the housing item is interactable, spawns and attach an interaction actor
  ;;[1 1 1] Overriden in child blueprint
)

(event `InteractionEvent`
  ;[1 1 1] If the housing item is interactable, spawns and attach an interaction actor
  ;;[1 1 1] Overriden in child blueprint
)

(event `self.SM_HousingMesh.OnClicked`
  (params (TouchedComponent :type "PrimitiveComponent Object Reference") (ButtonPressed :type "Key Structure"))
  ;[1 1 1] On click
  (set `/Game/LS_Template/Blueprints/Systems/Core/Game/BP_LS_GameController.SelectedHouseItem` self (`/Game/LS_Template/Blueprints/Systems/Core/BPL_Functions.Get_LST_Controller`)))

(event `self.ReceiveTick`
  (params (DeltaSeconds :type "Float (single-precision)"))
  (bind (_iteminfo_itemrowname _iteminfo_itemname _iteminfo_itemdescription _iteminfo_itemtype _iteminfo_clothestype _iteminfo_itemrarity _iteminfo_itemicon _iteminfo_itemsound _iteminfo_simulatephysics_ _iteminfo_itemmesh _iteminfo_itemprice _iteminfo_itemamount _iteminfo_gaindetails _iteminfo_housingdetails) (break `/Game/LS_Template/Blueprints/Systems/Structures/Items/S_ItemInfo` (`self.ItemInfo`)))
  (bind _sm_housingmesh (`self.SM_HousingMesh`))
  (bind (_meshrotation_roll _meshrotation_pitch) (`KismetMathLibrary.BreakRotator` (`self.MeshRotation`)))
  (bind (_bblockinghit _binitialoverlap _time _distance _location _impactpoint _normal) (`GameplayStatics.BreakHitResult` (`PlayerController.GetHitResultUnderCursorForObjects` (`/Game/LS_Template/Blueprints/Systems/Core/BPL_Functions.Get_LST_Controller`) (`|MakeArray` "ObjectTypeQuery1" :!type "EObjectTypeQuery Enum") true)))
  (bind (_returnvalue_roll _returnvalue_pitch _returnvalue_yaw) (`KismetMathLibrary.BreakRotator` (`KismetMathLibrary.MakeRotFromX` _normal)))
  (bind _returnvalue (`KismetMathLibrary.MakeVector` (.x _location) (.y _location) (+ (.z _location) 2.0)))
  ;[1 1 1] Event tick. Used for moving the item around
  (if (`.WallItem?_6_C5E5A9D743B25C281B3AA4AC2D4D0D46` (break `/Game/LS_Template/Blueprints/Systems/Structures/Housing/S_HousingDetails` _iteminfo_housingdetails))
    (`self.DetectNormalForWallItems` _normal
      (:`false`
        (bind _output_get (set `self.MeshLocation` (select `bool` (`PlayerController.IsInputKeyDown` (`/Game/LS_Template/Blueprints/Systems/Core/BPL_Functions.Get_LST_Controller`) "LeftShift") :`false` _returnvalue :`true` (`self.CalculateGridPosition` _returnvalue))))
        (`SceneComponent.K2_SetWorldLocation` _sm_housingmesh _output_get false false)
        (`SceneComponent.K2_SetWorldRotation` _sm_housingmesh (`KismetMathLibrary.MakeRotator` _meshrotation_roll _meshrotation_pitch _returnvalue_yaw) false false)
        (set `self.MeshRotation` (`SceneComponent.RelativeRotation` _sm_housingmesh))))
    (else
      (bind _outhit (`KismetSystemLibrary.LineTraceSingle` (`KismetMathLibrary.MakeVector` (.x _location) (.y _location) (+ (.z _location) 300.0)) (`KismetMathLibrary.MakeVector` (.x _location) (.y _location) (- (.z _location) 100.0)) "TraceTypeQuery1" false (`|MakeArray` self :!type "Actor Object Reference")))
      (bind (_bblockinghit_2 _binitialoverlap_2 _time_2 _distance_2 _location_2) (`GameplayStatics.BreakHitResult` _outhit))
      (if _bblockinghit_2
        (bind _output_get_2 (set `self.MeshLocation` (select `bool` (`PlayerController.IsInputKeyDown` (`/Game/LS_Template/Blueprints/Systems/Core/BPL_Functions.Get_LST_Controller`) "LeftShift") :`false` _location_2 :`true` (`self.CalculateGridPosition` _location_2))))
        (`SceneComponent.K2_SetWorldLocation` (`self.SM_HousingMesh`) _output_get_2 false false)))))

(fn `CalculateGridPosition`
  (params (CurrentLocation :type "Vector Structure"))
  (returns (GridLocation :type "Vector Structure"))
  (bind _gridsize_z (`self.GridSize_Z`))
  (bind _gridsize_x (`self.GridSize_X`))
  (bind _gridsize_y (`self.GridSize_Y`))
  (return (`KismetMathLibrary.MakeVector` (`KismetMathLibrary.Conv_IntToDouble` (* (`KismetMathLibrary.Round` (/ (.x CurrentLocation) (`KismetMathLibrary.Conv_IntToDouble` _gridsize_x))) _gridsize_x)) (`KismetMathLibrary.Conv_IntToDouble` (* (`KismetMathLibrary.Round` (/ (.y CurrentLocation) (`KismetMathLibrary.Conv_IntToDouble` _gridsize_y))) _gridsize_y)) (`KismetMathLibrary.Conv_IntToDouble` (* (`KismetMathLibrary.Round` (/ (.z CurrentLocation) (`KismetMathLibrary.Conv_IntToDouble` _gridsize_z))) _gridsize_z)))))

(fn `DisablePawnCollisionChannel`
  (params (`Disable?` :type Boolean))
  (`PrimitiveComponent.SetCollisionResponseToChannel` (`self.SM_HousingMesh`) "ECC_Pawn" (select `bool` `Disable?` :`false` "ECR_Block" :`true` "ECR_Ignore" :!type "ECollisionResponse Enum"))
  (return))

(fn `RotateMesh`
  (params (AxisValue :type "Float (double-precision)"))
  (bind _sm_housingmesh (`self.SM_HousingMesh`))
  (`SceneComponent.K2_AddLocalRotation` _sm_housingmesh (`KismetMathLibrary.MakeRotator` 0.0 0.0 (* AxisValue (`self.RotationSpeed`))) false false)
  (set `self.MeshRotation` (`SceneComponent.RelativeRotation` _sm_housingmesh))
  (return))

(fn `RotateWallMesh`
  (params (AxisValue :type "Float (double-precision)"))
  (bind _sm_housingmesh (`self.SM_HousingMesh`))
  (`SceneComponent.K2_AddLocalRotation` _sm_housingmesh (`KismetMathLibrary.MakeRotator` (* AxisValue (`self.RotationSpeed`))) false false)
  (set `self.MeshRotation` (`SceneComponent.RelativeRotation` _sm_housingmesh))
  (return))

(fn `SetActorTick`
  (params (`TickEnabled?` :type Boolean))
  (`self.SetActorTickEnabled` `TickEnabled?`)
  (return))

(fn `SetInteractionDefaults`
  (bind _interactionactor (`self.InteractionActor`))
  (bind (_iteminfo_itemrowname _iteminfo_itemname _iteminfo_itemdescription _iteminfo_itemtype _iteminfo_clothestype _iteminfo_itemrarity _iteminfo_itemicon _iteminfo_itemsound _iteminfo_simulatephysics_ _iteminfo_itemmesh) (break `/Game/LS_Template/Blueprints/Systems/Structures/Items/S_ItemInfo` (`self.ItemInfo`)))
  (`/Game/LS_Template/Blueprints/Interaction/Core/BP_InteractionActor.SetWidget` _interactionactor _iteminfo_itemname false 0 0)
  (`/Game/LS_Template/Blueprints/Interaction/Core/BP_InteractionActor.HandleInteractionShape` _interactionactor "NewEnumerator0" (* (`.SphereRadius` (`KismetMathLibrary.BreakBoxSphereBounds` (`StaticMesh.GetBounds` _iteminfo_itemmesh))) 1.2) (10.0 10.0 10.0) 96.0 42.0)
  (return))

(fn `SetOutline?`
  (params (`Outline?` :type Boolean))
  (if (`/Game/LS_Template/Blueprints/Systems/Core/LS_Instance.UseMeshOutline?` (`/Game/LS_Template/Blueprints/Systems/Core/BPL_Functions.Get_LST_Instance`))
    (`MaterialInstanceDynamic.SetVectorParameterValue` (`/Game/LS_Template/Blueprints/Interaction/Core/BPC_Interaction.OutlineDynamat` (`/Game/LS_Template/Blueprints/Systems/Core/Game/BP_LS_GameController.BPC_Interaction` (`/Game/LS_Template/Blueprints/Systems/Core/BPL_Functions.Get_LST_Controller`))) "OutlineColor" (struct :`R` 0.147275 :`G` 0.994792 :`B` 0.077031 :`A` 1.0))
    (`PrimitiveComponent.SetRenderCustomDepth` (`self.SM_HousingMesh`) `Outline?`)
    (return)))

(fn `UserConstructionScript`
  (bind _sm_housingmesh (`self.SM_HousingMesh`))
  (bind (_iteminfo_itemrowname _iteminfo_itemname _iteminfo_itemdescription _iteminfo_itemtype _iteminfo_clothestype _iteminfo_itemrarity _iteminfo_itemicon _iteminfo_itemsound _iteminfo_simulatephysics_ _iteminfo_itemmesh) (break `/Game/LS_Template/Blueprints/Systems/Structures/Items/S_ItemInfo` (`self.ItemInfo`)))
  (`StaticMeshComponent.SetStaticMesh` _sm_housingmesh _iteminfo_itemmesh)
  (`SceneComponent.K2_SetRelativeRotation` _sm_housingmesh (`self.MeshRotation`) false false)
  (`SceneComponent.K2_SetWorldLocation` _sm_housingmesh (`self.MeshLocation`) false false))