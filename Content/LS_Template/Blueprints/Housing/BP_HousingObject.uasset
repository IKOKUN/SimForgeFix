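; Placeable furniture actor for the housing system, taking its mesh from FurnitureItemInfo and registering as the controller's selected item when clicked.
; While Clicked, Tick moves it under the cursor: wall items align to the surface normal and skip horizontal faces, others use a downward trace, with Left Shift grid snapping.
; Interactable items spawn an attached BP_InteractionActor that toggles the outline; its interaction event is an empty stub.
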(event `self.ReceiveBeginPlay`
  (if (`.HousingInteractable?_1_54ECE45E462C0AAB003010B6A52186B5` (break `/Game/LS_Template/Blueprints/Systems/Structures/Housing/S_HousingDetails` (`.HousingDetails_87_FC11AFE04E261E465243BA98EE4F7524` (break `/Game/LS_Template/Blueprints/Systems/Structures/Items/S_ItemInfo` (`self.FurnitureItemInfo`)))))
    (bind _returnvalue (`|SpawnActorFromClass` "/Game/LS_Template/Blueprints/Interaction/Core/BP_InteractionActor.BP_InteractionActor_C" (`KismetMathLibrary.MakeTransform` (`PrimitiveComponent.GetCenterOfMass` (`self.SM_Furniture`) "None")) "Undefined" "MultiplyWithRoot" null "NewEnumerator0" null))
    (bind _output_get (set `self.Interactor Actor` _returnvalue))
    (`self.K2_AttachToComponent` _output_get (`self.SM_Furniture`) "None" "KeepRelative" "KeepRelative" "KeepRelative" true)
    (add `/Game/LS_Template/Blueprints/Interaction/Core/BP_InteractionActor.OnSetUseable` (`self.Interactor Actor`) (delegate `OnSetUseable`))
    (add `/Game/LS_Template/Blueprints/Interaction/Core/BP_InteractionActor.OnSetUnuseable` (`self.Interactor Actor`) (delegate `OnSetUnuseable`))
    (add `/Game/LS_Template/Blueprints/Interaction/Core/BP_InteractionActor.OnInteraction` (`self.Interactor Actor`) (delegate `InteractionEvent`))
    (add `self.OnActorEndOverlap` (`self.Interactor Actor`) (delegate `OnEndOverlap`))
    (`self.SetInteractionDefaults`)))

(event `OnSetUseable`
  (`self.SetOutline` true))

(event `OnSetUnuseable`
  (`self.SetOutline` false))

(event `OnEndOverlap` :!signature `self.OnActorEndOverlap`
  (params (OverlappedActor :type "Actor Object Reference") (OtherActor :type "Actor Object Reference")))

(event `InteractionEvent`)

(event `self.SM_Furniture.OnClicked`
  (params (TouchedComponent :type "PrimitiveComponent Object Reference") (ButtonPressed :type "Key Structure"))
  (set `/Game/LS_Template/Blueprints/Systems/Core/Game/BP_LS_GameController.SelectedHouseItem` self (`/Game/LS_Template/Blueprints/Systems/Core/BPL_Functions.Get_LST_Controller`)))

(event `self.ReceiveTick`
  (params (DeltaSeconds :type "Float (single-precision)"))
  (bind _sm_furniture (`self.SM_Furniture`))
  (bind (_meshrotation_roll _meshrotation_pitch) (`KismetMathLibrary.BreakRotator` (`self.MeshRotation`)))
  (bind (_furnitureiteminfo_itemrowname _furnitureiteminfo_itemname _furnitureiteminfo_itemdescription _furnitureiteminfo_itemtype _furnitureiteminfo_clothestype _furnitureiteminfo_itemrarity _furnitureiteminfo_itemicon _furnitureiteminfo_itemsound _furnitureiteminfo_simulatephysics_ _furnitureiteminfo_itemmesh _furnitureiteminfo_itemskeletalmesh _furnitureiteminfo_itemprice _furnitureiteminfo_itemamount _furnitureiteminfo_gaindetails _furnitureiteminfo_housingdetails) (break `/Game/LS_Template/Blueprints/Systems/Structures/Items/S_ItemInfo` (`self.FurnitureItemInfo`)))
  (bind (_bblockinghit _binitialoverlap _time _distance _location _impactpoint _normal) (`GameplayStatics.BreakHitResult` (`PlayerController.GetHitResultUnderCursorForObjects` (`/Game/LS_Template/Blueprints/Systems/Core/BPL_Functions.Get_LST_Controller`) (`|MakeArray` "ObjectTypeQuery1" :!type "EObjectTypeQuery Enum") true)))
  (bind (_returnvalue_roll _returnvalue_pitch _returnvalue_yaw) (`KismetMathLibrary.BreakRotator` (`KismetMathLibrary.MakeRotFromX` _normal)))
  (bind _returnvalue (`KismetMathLibrary.MakeVector` (.x _location) (.y _location) (+ (.z _location) 2.0)))
  ;[1 1 1] Event tick. Used for moving the item around
  (if (`self.Clicked?`)
    (if (`.WallItem?_6_C5E5A9D743B25C281B3AA4AC2D4D0D46` (break `/Game/LS_Template/Blueprints/Systems/Structures/Housing/S_HousingDetails` _furnitureiteminfo_housingdetails))
      (`self.DetectNormalForWallItems` _normal
        (:`false`
          (bind _output_get (set `self.MeshLocation` (select `bool` (`PlayerController.IsInputKeyDown` (`/Game/LS_Template/Blueprints/Systems/Core/BPL_Functions.Get_LST_Controller`) "LeftShift") :`false` _returnvalue :`true` (`self.CalculateGridPosition` _returnvalue))))
          (`SceneComponent.K2_SetWorldLocation` _sm_furniture _output_get false false)
          (`SceneComponent.K2_SetWorldRotation` _sm_furniture (`KismetMathLibrary.MakeRotator` _meshrotation_roll _meshrotation_pitch _returnvalue_yaw) false false)
          (set `self.MeshRotation` (`SceneComponent.RelativeRotation` _sm_furniture))))
      (else
        (bind _outhit (`KismetSystemLibrary.LineTraceSingle` (`KismetMathLibrary.MakeVector` (.x _location) (.y _location) (+ (.z _location) 300.0)) (`KismetMathLibrary.MakeVector` (.x _location) (.y _location) (- (.z _location) 100.0)) "TraceTypeQuery1" false (`|MakeArray` self :!type "Actor Object Reference")))
        (bind (_bblockinghit_2 _binitialoverlap_2 _time_2 _distance_2 _location_2) (`GameplayStatics.BreakHitResult` _outhit))
        (if _bblockinghit_2
          (bind _output_get_2 (set `self.MeshLocation` (select `bool` (`PlayerController.IsInputKeyDown` (`/Game/LS_Template/Blueprints/Systems/Core/BPL_Functions.Get_LST_Controller`) "LeftShift") :`false` _location_2 :`true` (`self.CalculateGridPosition` _location_2))))
          (`SceneComponent.K2_SetWorldLocation` (`self.SM_Furniture`) _output_get_2 false false))))))

(fn `CalculateGridPosition`
  (params (CurrentLocation :type "Vector Structure"))
  (returns (GridLocation :type "Vector Structure"))
  (bind _gridsize_z (`self.GridSize_Z`))
  (bind _gridsize_x (`self.GridSize_X`))
  (bind _gridsize_y (`self.GridSize_Y`))
  (return (`KismetMathLibrary.MakeVector` (`KismetMathLibrary.Conv_IntToDouble` (* (`KismetMathLibrary.Round` (/ (.x CurrentLocation) (`KismetMathLibrary.Conv_IntToDouble` _gridsize_x))) _gridsize_x)) (`KismetMathLibrary.Conv_IntToDouble` (* (`KismetMathLibrary.Round` (/ (.y CurrentLocation) (`KismetMathLibrary.Conv_IntToDouble` _gridsize_y))) _gridsize_y)) (`KismetMathLibrary.Conv_IntToDouble` (* (`KismetMathLibrary.Round` (/ (.z CurrentLocation) (`KismetMathLibrary.Conv_IntToDouble` _gridsize_z))) _gridsize_z)))))

(fn `DisablePawnCollisionChannel`
  (params (`Disable?` :type Boolean))
  (`PrimitiveComponent.SetCollisionResponseToChannel` (`self.SM_Furniture`) "ECC_Pawn" (select `bool` `Disable?` :`false` "ECR_Block" :`true` "ECR_Ignore" :!type "ECollisionResponse Enum"))
  (return))

(fn `RotateMesh`
  (params (AxisValue :type "Float (double-precision)"))
  (bind _sm_furniture (`self.SM_Furniture`))
  (`SceneComponent.K2_AddLocalRotation` _sm_furniture (`KismetMathLibrary.MakeRotator` 0.0 0.0 (* AxisValue (`self.RotationSpeed`))) false false)
  (set `self.MeshRotation` (`SceneComponent.RelativeRotation` _sm_furniture))
  (return))

(fn `RotateWallMesh`
  (params (AxisValue :type "Float (double-precision)"))
  (bind _sm_furniture (`self.SM_Furniture`))
  (`SceneComponent.K2_AddLocalRotation` _sm_furniture (`KismetMathLibrary.MakeRotator` (* AxisValue (`self.RotationSpeed`))) false false)
  (set `self.MeshRotation` (`SceneComponent.RelativeRotation` _sm_furniture))
  (return))

(fn `SetActorTick`
  (params (`TickEnabled?` :type Boolean))
  (`self.SetActorTickEnabled` `TickEnabled?`)
  (return))

(fn `SetInteractionDefaults`
  (bind (_furnitureiteminfo_itemrowname _furnitureiteminfo_itemname _furnitureiteminfo_itemdescription _furnitureiteminfo_itemtype _furnitureiteminfo_clothestype _furnitureiteminfo_itemrarity _furnitureiteminfo_itemicon _furnitureiteminfo_itemsound _furnitureiteminfo_simulatephysics_ _furnitureiteminfo_itemmesh) (break `/Game/LS_Template/Blueprints/Systems/Structures/Items/S_ItemInfo` (`self.FurnitureItemInfo`)))
  (bind _interactor_actor (`self.Interactor Actor`))
  (`/Game/LS_Template/Blueprints/Interaction/Core/BP_InteractionActor.SetWidget` _interactor_actor _furnitureiteminfo_itemname false 0 0)
  (`/Game/LS_Template/Blueprints/Interaction/Core/BP_InteractionActor.HandleInteractionShape` _interactor_actor "NewEnumerator0" (* (`.SphereRadius` (`KismetMathLibrary.BreakBoxSphereBounds` (`StaticMesh.GetBounds` _furnitureiteminfo_itemmesh))) 1.2) (10.0 10.0 10.0) 96.0 42.0))

(fn `SetOutline`
  (params (`Outline?` :type Boolean))
  (if (`/Game/LS_Template/Blueprints/Systems/Core/LS_Instance.UseMeshOutline?` (`/Game/LS_Template/Blueprints/Systems/Core/BPL_Functions.Get_LST_Instance`))
    (`MaterialInstanceDynamic.SetVectorParameterValue` (`/Game/LS_Template/Blueprints/Interaction/Core/BPC_Interaction.OutlineDynamat` (`/Game/LS_Template/Blueprints/Systems/Core/Game/BP_LS_GameController.BPC_Interaction` (`/Game/LS_Template/Blueprints/Systems/Core/BPL_Functions.Get_LST_Controller`))) "OutlineColor" (struct :`R` 0.042449 :`G` 0.994792 :`A` 1.0))
    (`PrimitiveComponent.SetRenderCustomDepth` (`self.SM_Furniture`) `Outline?`)))

(fn `UserConstructionScript`
  (bind _sm_furniture (`self.SM_Furniture`))
  (`StaticMeshComponent.SetStaticMesh` _sm_furniture (`.ItemMesh_68_73B87E0A4F870D302450A0900AFD3E1A` (break `/Game/LS_Template/Blueprints/Systems/Structures/Items/S_ItemInfo` (`self.FurnitureItemInfo`))))
  (`SceneComponent.K2_SetRelativeRotation` _sm_furniture (`self.MeshRotation`) false false)
  (`SceneComponent.K2_SetWorldLocation` _sm_furniture (`self.MeshLocation`) false false))