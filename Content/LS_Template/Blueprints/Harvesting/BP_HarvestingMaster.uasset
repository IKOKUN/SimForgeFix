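; BP_HarvestingMaster is a base actor for harvestable objects that grant an inventory item when interacted with.
; A child BP_InteractionActor, configured in the construction script for shape, location and prompt, supplies the interaction and useable events.
; Becoming useable toggles a green custom-depth outline on the mesh if the game instance enables outlines.
; Harvesting adds the item and destroys the actor, or shows a HUD message when no inventory slot is free.
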(event `self.ReceiveBeginPlay`
  (bind _interactionactor (`self.InteractionActor`))
  (`/Game/LS_Template/Blueprints/Interaction/Core/BP_InteractionActor.SetWidget` _interactionactor (`self.HarvestName`) false 0 0)
  (add `/Game/LS_Template/Blueprints/Interaction/Core/BP_InteractionActor.OnInteraction` _interactionactor (delegate `OnInteractionEvent`))
  (add `/Game/LS_Template/Blueprints/Interaction/Core/BP_InteractionActor.OnSetUseable` _interactionactor (delegate `EventOnUseable`))
  (add `/Game/LS_Template/Blueprints/Interaction/Core/BP_InteractionActor.OnSetUnuseable` _interactionactor (delegate `EventOnUnuseable`)))

(event `EventOnUseable`
  (`self.SetOulineMesh` true))

(event `EventOnUnuseable`
  (`self.SetOulineMesh` false))

(event `OnInteractionEvent`
  (`self.OnHarvest`))

(event `OnHarvest`
  (bind _success_ (`/Game/LS_Template/Blueprints/Systems/Core/BPL_Functions.SearchEmptySlot`))
  (if _success_
    (`/Game/LS_Template/Blueprints/Systems/Core/BPL_Functions.AddItemToInventory` (`self.HarvestedItemRowName`) (`self.HarvestedAmount`))
    (`self.K2_DestroyActor`)
    (else
      (`/Game/LS_Template/Blueprints/Systems/Core/BPL_Functions.DisplayHUD_Message` false "Your inventory is full !" (struct :`R` 0.994792 :`A` 1.0)))))

(fn `SetOulineMesh`
  (params (`Outline?` :type Boolean))
  (if (`/Game/LS_Template/Blueprints/Systems/Core/LS_Instance.UseMeshOutline?` (`/Game/LS_Template/Blueprints/Systems/Core/BPL_Functions.Get_LST_Instance`))
    (`MaterialInstanceDynamic.SetVectorParameterValue` (`/Game/LS_Template/Blueprints/Interaction/Core/BPC_Interaction.OutlineDynamat` (`/Game/LS_Template/Blueprints/Systems/Core/Game/BP_LS_GameController.BPC_Interaction` (`/Game/LS_Template/Blueprints/Systems/Core/BPL_Functions.Get_LST_Controller`))) "OutlineColor" (struct :`R` 0.147275 :`G` 0.994792 :`B` 0.077031 :`A` 1.0))
    (`PrimitiveComponent.SetRenderCustomDepth` (`self.SM_HarvestMesh`) `Outline?`)
    (return)
    (else
      (return))))

(fn `UserConstructionScript`
  (bind _interactionactor (`self.InteractionActor`))
  (bind _asbp_interaction_actor (cast `/Game/LS_Template/Blueprints/Interaction/Core/BP_InteractionActor` (`ChildActorComponent.ChildActor` (`self.ChildActor`))))
  (set `self.InteractionActor` _asbp_interaction_actor)
  (`/Game/LS_Template/Blueprints/Interaction/Core/BP_InteractionActor.HandleInteractionShape` _interactionactor (`self.InteractionShape`) (`self.SphereRadius`) (`self.BoxExtent`) (`self.CapsuleHalfHeight`) (`self.CapsuleRadius`))
  (`self.K2_SetActorRelativeLocation` _interactionactor (`self.InteractionLocation`) false false)
  (`SceneComponent.K2_SetRelativeLocation` (`/Game/LS_Template/Blueprints/Interaction/Core/BP_InteractionActor.Widget` _interactionactor) (`self.PromptLocation`) false false))