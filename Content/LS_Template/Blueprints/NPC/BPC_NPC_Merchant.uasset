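; Merchant NPC that opens a shop menu for the player on interaction, extending a parent NPC Blueprint.
; Interaction toggles the roaming timer, shows the inventory, optionally blends the camera to the merchant, disables player movement and creates W_MerchantMenu with the offered items.
; ExitMenu restores camera, walking, roaming and prompt.
; If the inventory is visible, it toggles that HUD and clears interaction flags after a short delay.
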(event `self.ReceiveBeginPlay`
  (`parent.ReceiveBeginPlay`)
  (`/Game/LS_Template/Blueprints/Interaction/Core/BP_InteractionActor.SetWidget` (`self.InteractionActor`) (`self.NPC_Name`) false 0 0))

(event `self.OnInteractionEvent`
  (`parent.OnInteractionEvent`)
  (`self.RoamingTimerHandle` true)
  (`self.DisplayMerchantMenu`))

(event `DisplayMerchantMenu`
  (bind _w_playerhud (`/Game/LS_Template/Blueprints/Systems/Core/BPL_Functions.Get_LST_PlayerHUD`))
  ;[1 1 1] Is the HUD visible ? If false, then display it
  (if (not (`/Game/LS_Template/Blueprints/UI/W_PlayerHUD.IsInventoryVisible` _w_playerhud))
    (`/Game/LS_Template/Blueprints/UI/W_PlayerHUD.DisplayHUD` _w_playerhud false true))
  ;[1 1 1] Use View blend ? If true, then blend view
  (if (`self.UseViewBlend?`)
    (`PlayerController.SetViewTargetWithBlend` (`/Game/LS_Template/Blueprints/Systems/Core/BPL_Functions.Get_LST_Controller`) self (`self.BlendTime`) "VTBlend_Linear" 0.0 false))
  ;[1 1 1] Disable movement during interactions
  (`CharacterMovementComponent.DisableMovement` (`Character.CharacterMovement` (`GameplayStatics.GetPlayerCharacter` 0)))
  ;[1 1 1] Creates and displays Merchant menu
  (bind _returnvalue (`|CreateWidget` "/Game/LS_Template/Blueprints/UI/NPC/Merchants/W_MerchantMenu.W_MerchantMenu_C" null (`self.OfferedItems`) self))
  (`UserWidget.AddToViewport` _returnvalue 0))

(event `ExitMenu`
  (bind _w_playerhud (`/Game/LS_Template/Blueprints/Systems/Core/BPL_Functions.Get_LST_PlayerHUD`))
  (`/Game/LS_Template/Blueprints/Interaction/Core/BP_InteractionActor.HidePrompt` (`self.InteractionActor`) true)
  (if (`self.UseViewBlend?`)
    (`PlayerController.SetViewTargetWithBlend` (`/Game/LS_Template/Blueprints/Systems/Core/BPL_Functions.Get_LST_Controller`) (`GameplayStatics.GetPlayerCharacter` 0) 0.75 "VTBlend_Linear" 0.0 false))
  (`CharacterMovementComponent.SetMovementMode` (`Character.CharacterMovement` (`GameplayStatics.GetPlayerCharacter` 0)) "MOVE_Walking" 0)
  (`self.RoamingTimerHandle` false)
  (if (`/Game/LS_Template/Blueprints/UI/W_PlayerHUD.IsInventoryVisible` _w_playerhud)
    (`/Game/LS_Template/Blueprints/UI/W_PlayerHUD.DisplayHUD` _w_playerhud false true)
    (`KismetSystemLibrary.Delay` 0.75)
    (set `/Game/LS_Template/Blueprints/Systems/Core/Game/BP_LS_GameController.IsInteractingWithNPC?` false (`/Game/LS_Template/Blueprints/Systems/Core/BPL_Functions.Get_LST_Controller`))
    (set `self.bHasInteract` false))
  (`/Game/LS_Template/Blueprints/Systems/Core/BPL_Functions.SetInteractTextWidget` (`self.Interact Text`))
  (`/Game/LS_Template/Blueprints/Systems/Core/BPL_Functions.SetInteractWidgetVisibility` "SelfHitTestInvisible"))

(fn `UserConstructionScript`)