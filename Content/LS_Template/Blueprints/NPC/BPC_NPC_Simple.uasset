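; Simple NPC Blueprint that shows a random one-line message when the player interacts with it.
; Extends a parent NPC class, picking text from DialogLines at BeginPlay and on each interaction and pushing it to the InteractionActor widget.
; Interaction pauses optional roaming and immediately clears the controller's IsInteractingWithNPC flag.
; Becoming unuseable toggles the prompt back and resumes roaming.
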(event `self.ReceiveBeginPlay`
  (bind _interactionactor (`self.InteractionActor`))
  (`parent.ReceiveBeginPlay`)
  (`/Game/LS_Template/Blueprints/Interaction/Core/BP_InteractionActor.SetWidget` _interactionactor (`self.SetRandomMessage`) false 0 0)
  (`/Game/LS_Template/Blueprints/Interaction/Core/BP_InteractionActor.HidePrompt` _interactionactor false))

(event `self.OnInteractionEvent`
  (bind _interactionactor (`self.InteractionActor`))
  ;[1 1 1] Pause roaming timer after interaction
  (if (`self.ShouldRoam?`)
    (`self.RoamingTimerHandle` true))
  (`/Game/LS_Template/Blueprints/Interaction/Core/BP_InteractionActor.HidePrompt` _interactionactor true)
  (`/Game/LS_Template/Blueprints/Interaction/Core/BP_InteractionActor.SetWidget` _interactionactor (`self.SetRandomMessage`) false 0 0)
  (`parent.OnInteractionEvent`)
  (set `/Game/LS_Template/Blueprints/Systems/Core/Game/BP_LS_GameController.IsInteractingWithNPC?` false (`/Game/LS_Template/Blueprints/Systems/Core/BPL_Functions.Get_LST_Controller`)))

(event `self.EventOnUseable`
  (`self.SetMeshOutline` false))

(event `self.EventOnUnuseable`
  (`self.SetMeshOutline` false)
  (`/Game/LS_Template/Blueprints/Interaction/Core/BP_InteractionActor.HidePrompt` (`self.InteractionActor`) false)
  ;[1 1 1] Unpause roaming timer after interaction
  (if (`self.ShouldRoam?`)
    (`self.RoamingTimerHandle` false)))

(fn `SetRandomMessage`
  (returns (SelectedMessage :type Text))
  (bind _dialoglines (`self.DialogLines`))
  (return (`|GetArrayItem` _dialoglines (`KismetMathLibrary.RandomIntegerInRange` 0 (`KismetArrayLibrary.Array_LastIndex` _dialoglines)))))

(fn `UserConstructionScript`
  (`parent.UserConstructionScript`))