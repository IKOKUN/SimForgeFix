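; Base Blueprint for interactable NPC-style actors that turn to face the player when used and flag the controller as interacting with an NPC.
; The construction script configures a child BP_InteractionActor's trigger shape, location and prompt, and positions a camera.
; BeginPlay binds its interaction and useable events, which also toggle an optional custom-depth outline with a configurable color.
; ExitMenu is an empty event.
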(event `self.ReceiveBeginPlay`
  (bind _interactionactor (`self.InteractionActor`))
  (add `/Game/LS_Template/Blueprints/Interaction/Core/BP_InteractionActor.OnInteraction` _interactionactor (delegate `OnInteractionEvent`))
  (add `/Game/LS_Template/Blueprints/Interaction/Core/BP_InteractionActor.OnSetUseable` _interactionactor (delegate `EventOnUseable`))
  (add `/Game/LS_Template/Blueprints/Interaction/Core/BP_InteractionActor.OnSetUnuseable` _interactionactor (delegate `EventOnUnuseable`)))

(event `EventOnUseable`
  (`self.SetMeshOutline` true))

(event `EventOnUnuseable`
  (`self.SetMeshOutline` false))

(event `OnInteractionEvent`
  (bind (_returnvalue_roll _returnvalue_pitch _returnvalue_yaw) (`KismetMathLibrary.BreakRotator` (`KismetMathLibrary.FindLookAtRotation` (`self.K2_GetActorLocation` (`GameplayStatics.GetPlayerCharacter` 0)) (`self.K2_GetActorLocation` self))))
  ;[1 1 1] Overriden in child blueprints
  ;[1 1 1] Make the NPC face the player character
  (set `/Game/LS_Template/Blueprints/Systems/Core/Game/BP_LS_GameController.IsInteractingWithNPC?` true (`/Game/LS_Template/Blueprints/Systems/Core/BPL_Functions.Get_LST_Controller`))
  (`self.K2_SetActorRotation` (`KismetMathLibrary.MakeRotator` 0.0 0.0 (- _returnvalue_yaw 180.0))))

(event `Exit Menu`)

(fn `SetMeshOutline`
  (params (`Outline?` :type Boolean))
  (if (`/Game/LS_Template/Blueprints/Systems/Core/LS_Instance.UseMeshOutline?` (`/Game/LS_Template/Blueprints/Systems/Core/BPL_Functions.Get_LST_Instance`))
    (`MaterialInstanceDynamic.SetVectorParameterValue` (`/Game/LS_Template/Blueprints/Interaction/Core/BPC_Interaction.OutlineDynamat` (`/Game/LS_Template/Blueprints/Systems/Core/Game/BP_LS_GameController.BPC_Interaction` (`/Game/LS_Template/Blueprints/Systems/Core/BPL_Functions.Get_LST_Controller`))) "OutlineColor" (`self.OutlineColor`))
    (`PrimitiveComponent.SetRenderCustomDepth` (`self.Cube`) `Outline?`)
    (return)))

(fn `UserConstructionScript`
  (bind _interactionactor (`self.InteractionActor`))
  (bind _asbp_interaction_actor (cast `/Game/LS_Template/Blueprints/Interaction/Core/BP_InteractionActor` (`ChildActorComponent.ChildActor` (`self.ChildActor`))))
  (set `self.InteractionActor` _asbp_interaction_actor)
  (`/Game/LS_Template/Blueprints/Interaction/Core/BP_InteractionActor.HandleInteractionShape` _interactionactor (`self.InteractionShape`) (`self.SphereRadius`) (`self.BoxExtent`) (`self.CapsuleHalfHeight`) (`self.CapsuleRadius`))
  (`self.K2_SetActorRelativeLocation` _interactionactor (`self.InteractionLocation`) false false)
  (`SceneComponent.K2_SetRelativeLocation` (`/Game/LS_Template/Blueprints/Interaction/Core/BP_InteractionActor.Widget` _interactionactor) (`self.PromptLocation`) false false)
  (`SceneComponent.K2_SetRelativeLocationAndRotation` (`self.Camera`) (`self.CameraLocation`) (`self.CameraRotation`) false false))