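; Base NPC Blueprint for child NPCs, providing player interaction, optional mesh outlining and optional roaming.
; The construction script configures a child BP_InteractionActor's shape and prompt, plus the camera transform.
; Interaction events toggle a custom-depth outline and, on interaction, flag the controller and turn the NPC toward the player.
; A looping timer issues AI moves to random reachable points, with a function to halt movement and pause or resume it.
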(event `self.ReceiveBeginPlay`
  (bind _interactionactor (`self.InteractionActor`))
  (add `/Game/LS_Template/Blueprints/Interaction/Core/BP_InteractionActor.OnInteraction` _interactionactor (delegate `OnInteractionEvent`))
  (add `/Game/LS_Template/Blueprints/Interaction/Core/BP_InteractionActor.OnSetUseable` _interactionactor (delegate `EventOnUseable`))
  (add `/Game/LS_Template/Blueprints/Interaction/Core/BP_InteractionActor.OnSetUnuseable` _interactionactor (delegate `EventOnUnuseable`))
  (if (`self.ShouldRoam?`)
    (bind _returnvalue (`KismetSystemLibrary.K2_SetTimerDelegate` (delegate `BeginMoving`) 5.0 true))
    (set `self.RoamingTimer` _returnvalue)))

(event `EventOnUseable`
  (`self.SetMeshOutline` true))

(event `EventOnUnuseable`
  (`self.SetMeshOutline` false))

(event `OnInteractionEvent`
  (bind (_returnvalue_roll _returnvalue_pitch _returnvalue_yaw) (`KismetMathLibrary.BreakRotator` (`KismetMathLibrary.FindLookAtRotation` (`self.K2_GetActorLocation` (`GameplayStatics.GetPlayerCharacter` 0)) (`self.K2_GetActorLocation` self))))
  ;[1 1 1] Overriden in child blueprints
  ;[1 1 1] Make the NPC face the player character
  (set `/Game/LS_Template/Blueprints/Systems/Core/Game/BP_LS_GameController.IsInteractingWithNPC?` true (`/Game/LS_Template/Blueprints/Systems/Core/BPL_Functions.Get_LST_Controller`))
  (`self.K2_SetActorRotation` (`KismetMathLibrary.MakeRotator` 0.0 0.0 (- _returnvalue_yaw 180.0))))

(event `BeginMoving`
  ;[1 0 0] Roaming example
  (`|AIMoveTo` self (`NavigationSystemV1.K2_GetRandomReachablePointInRadius` (`self.K2_GetActorLocation`) 1000.0 null null) null))

(fn `RoamingTimerHandle`
  (params (`PauseTimer?` :type Boolean))
  (bind _charactermovement (`self.CharacterMovement`))
  (if (`KismetSystemLibrary.K2_IsValidTimerHandle` (`self.RoamingTimer`))
    (if (`NavMovementComponent.IsMovingOnGround` _charactermovement)
      (`MovementComponent.StopMovementImmediately` _charactermovement))
    (if `PauseTimer?`
      (`KismetSystemLibrary.K2_PauseTimerHandle` (`self.RoamingTimer`))
      (else
        (`KismetSystemLibrary.K2_UnPauseTimerHandle` (`self.RoamingTimer`))))
    (return)
    (else
      (return))))

(fn `SetMeshOutline`
  (params (`Outline?` :type Boolean))
  (if (`/Game/LS_Template/Blueprints/Systems/Core/LS_Instance.UseMeshOutline?` (`/Game/LS_Template/Blueprints/Systems/Core/BPL_Functions.Get_LST_Instance`))
    (`MaterialInstanceDynamic.SetVectorParameterValue` (`/Game/LS_Template/Blueprints/Interaction/Core/BPC_Interaction.OutlineDynamat` (`/Game/LS_Template/Blueprints/Systems/Core/Game/BP_LS_GameController.BPC_Interaction` (`/Game/LS_Template/Blueprints/Systems/Core/BPL_Functions.Get_LST_Controller`))) "OutlineColor" (`self.OutlineColor`))
    (`PrimitiveComponent.SetRenderCustomDepth` (`self.Mesh`) `Outline?`)
    (return)))

(fn `UserConstructionScript`
  (bind _interactionactor (`self.InteractionActor`))
  (bind _asbp_interaction_actor (cast `/Game/LS_Template/Blueprints/Interaction/Core/BP_InteractionActor` (`ChildActorComponent.ChildActor` (`self.ChildActor`))))
  (set `self.InteractionActor` _asbp_interaction_actor)
  (`/Game/LS_Template/Blueprints/Interaction/Core/BP_InteractionActor.HandleInteractionShape` _interactionactor (`self.InteractionShape`) (`self.SphereRadius`) (`self.BoxExtent`) (`self.CapsuleHalfHeight`) (`self.CapsuleRadius`))
  (`self.K2_SetActorRelativeLocation` _interactionactor (`self.InteractionLocation`) false false)
  (`SceneComponent.K2_SetRelativeLocation` (`/Game/LS_Template/Blueprints/Interaction/Core/BP_InteractionActor.Widget` _interactionactor) (`self.PromptLocation`) false false)
  (`SceneComponent.K2_SetRelativeLocationAndRotation` (`self.Camera`) (`self.CameraLocation`) (`self.CameraRotation`) false false))