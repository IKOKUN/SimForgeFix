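; Story NPC Blueprint that runs a dialog interaction, pausing roaming, freezing and hiding the player, and optionally blending the camera to itself.
; Construction loads NPC info from DT_NPC by row name and builds either a single mesh or master-posed multipart meshes.
; Dialog start refreshes info from the game instance's known-NPC list or registers the NPC there, then opens W_StoryNPC.
; ExitMenu restores camera, movement and input.
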(event `self.ReceiveBeginPlay`
  (bind (_npc_info_npcrowname _npc_info_alreadyknownnpc_ _npc_info_npcname) (break `/Game/LS_Template/Blueprints/Systems/Structures/NPC/S_NPC_Info` (`self.NPC_Info`)))
  (`parent.ReceiveBeginPlay`)
  (`/Game/LS_Template/Blueprints/Interaction/Core/BP_InteractionActor.SetWidget` (`self.InteractionActor`) _npc_info_npcname false 0 0))

(event `self.OnInteractionEvent`
  (`parent.OnInteractionEvent`)
  (`self.RoamingTimerHandle` true)
  (`self.StartDialog`))

(event `StartDialog`
  (bind _w_playerhud (`/Game/LS_Template/Blueprints/Systems/Core/BPL_Functions.Get_LST_PlayerHUD`))
  (bind (_npc_found_ _outnpc_info) (`self.CheckIfNPC_IsAlreadyKnown`))
  (bind _lst_controller (`/Game/LS_Template/Blueprints/Systems/Core/BPL_Functions.Get_LST_Controller`))
  (bind _w_storynpc (`self.W_StoryNPC`))
  ;[0.9948 0 0] Change the cast to your own character in here
  (`self.HidePlayerMesh?` true)
  ;[1 1 1] Is this NPC already known ?
  (if _npc_found_
    ;[1 1 1] If true, gets the freshest NPC Info from LST Instance
    (set `self.NPC_Info` _outnpc_info)
    (else
      ;[1 1 1] If flase, adds it to the known NPC in LST Instance
      (`KismetArrayLibrary.Array_AddUnique` (`/Game/LS_Template/Blueprints/Systems/Core/LS_Instance.KnownsNPC` (`/Game/LS_Template/Blueprints/Systems/Core/BPL_Functions.Get_LST_Instance`)) (`self.NPC_Info`))
      (`/Game/LS_Template/Blueprints/UI/W_PlayerHUD.UpdateAffectionBox` (`/Game/LS_Template/Blueprints/Systems/Core/BPL_Functions.Get_LST_PlayerHUD`))))
  ;[1 1 1] Is the HUD visible ? If false, then hide it
  (if (`/Game/LS_Template/Blueprints/UI/W_PlayerHUD.IsVisible?` _w_playerhud)
    (`/Game/LS_Template/Blueprints/UI/W_PlayerHUD.DisplayHUD` _w_playerhud false))
  ;[1 1 1] Use View blend ? If true, then blend view
  (if (`self.UseViewBlend?`)
    (`PlayerController.SetViewTargetWithBlend` (`/Game/LS_Template/Blueprints/Systems/Core/BPL_Functions.Get_LST_Controller`) self (`self.BlendTime`) "VTBlend_Linear" 0.0 false))
  ;[1 1 1] Disable movement during interactions
  (`CharacterMovementComponent.DisableMovement` (`Character.CharacterMovement` (`GameplayStatics.GetPlayerCharacter` 0)))
  ;[1 1 1] Creates and displays Story NPC widget
  (`/Engine/EditorBlueprintResources/StandardMacros.IsValid` _w_storynpc
    (:`Is Valid`
      (`/Game/LS_Template/Blueprints/UI/NPC/Story/W_StoryNPC.UpdateWidget` _w_storynpc))
    (:`Is Not Valid`
      (bind _returnvalue (`|CreateWidget` "/Game/LS_Template/Blueprints/UI/NPC/Story/W_StoryNPC.W_StoryNPC_C" null (`self.NPC_RowName`) self))
      (set `self.W_StoryNPC` _returnvalue)))
  (`UserWidget.AddToViewport` (`self.W_StoryNPC`) 0)
  (set `PlayerController.bShowMouseCursor` true _lst_controller)
  (`WidgetBlueprintLibrary.SetInputMode_UIOnlyEx` _lst_controller (`self.W_StoryNPC`)))

(event `ExitMenu`
  (bind _lst_controller (`/Game/LS_Template/Blueprints/Systems/Core/BPL_Functions.Get_LST_Controller`))
  ;[1 1 1] Called when exit NPC Story widget
  (`/Game/LS_Template/Blueprints/Interaction/Core/BP_InteractionActor.HidePrompt` (`self.InteractionActor`) true)
  (if (`self.UseViewBlend?`)
    (`PlayerController.SetViewTargetWithBlend` (`/Game/LS_Template/Blueprints/Systems/Core/BPL_Functions.Get_LST_Controller`) (`GameplayStatics.GetPlayerCharacter` 0) 0.75 "VTBlend_Linear" 0.0 false))
  (`CharacterMovementComponent.SetMovementMode` (`Character.CharacterMovement` (`GameplayStatics.GetPlayerCharacter` 0)) "MOVE_Walking" 0)
  (`self.HidePlayerMesh?` false)
  (set `PlayerController.bShowMouseCursor` false _lst_controller)
  (`WidgetBlueprintLibrary.SetInputMode_GameOnly` _lst_controller)
  (`KismetSystemLibrary.Delay` 0.75)
  (set `/Game/LS_Template/Blueprints/Systems/Core/Game/BP_LS_GameController.IsInteractingWithNPC?` false (`/Game/LS_Template/Blueprints/Systems/Core/BPL_Functions.Get_LST_Controller`))
  ;;[1 1 1] Unpause roaming timer after interaction
  (if (`self.ShouldRoam?`)
    (`self.RoamingTimerHandle` false)))

(fn `CheckIfNPC_IsAlreadyKnown`
  (returns (`NPC_Found?` :type Boolean) (OutNPC_Info :type "/Game/LS_Template/Blueprints/Systems/Structures/NPC/S_NPC_Info Structure"))
  (locals (`LocalFound?` :type Boolean) (FoundIndex :type Integer))
  (for (_array_element _array_index) (`/Game/LS_Template/Blueprints/Systems/Core/LS_Instance.KnownsNPC` (`/Game/LS_Template/Blueprints/Systems/Core/BPL_Functions.Get_LST_Instance`))
    (if (== (`.NPCRowName_26_772963274E2781E3AE1CB280D5E1328F` (break `/Game/LS_Template/Blueprints/Systems/Structures/NPC/S_NPC_Info` _array_element)) (`self.NPC_RowName`))
      (set `local.LocalFound?` true)
      (set `local.FoundIndex` _array_index)
      (break)))
  (return (`local.LocalFound?`) (`|GetArrayItem` (`/Game/LS_Template/Blueprints/Systems/Core/LS_Instance.KnownsNPC` (`/Game/LS_Template/Blueprints/Systems/Core/BPL_Functions.Get_LST_Instance`)) (`local.FoundIndex`))))

(fn `HidePlayerMesh?`
  (params (Hide :type Boolean))
  (bind _asthird_person_character (cast `/Game/LS_Template/EpicContent/CharacterExampleContent/ThirdPersonCharacter` (`GameplayStatics.GetPlayerCharacter` 0)))
  (`SceneComponent.SetHiddenInGame` (`Character.Mesh` _asthird_person_character) Hide false))

(fn `SetFeetMesh`
  (params (`Mesh Info` :type "/Game/LS_Template/Blueprints/Systems/Structures/Meshes/S_MeshInfo Structure"))
  (bind (_skeletalmesh _meshmaterials) (break `/Game/LS_Template/Blueprints/Systems/Structures/Meshes/S_MeshInfo` `Mesh Info`))
  (bind _sk_feetmesh (`self.SK_FeetMesh`))
  (`SkinnedMeshComponent.SetSkinnedAssetAndUpdate` _sk_feetmesh _skeletalmesh true)
  (for (_array_element _array_index) _meshmaterials
    (`PrimitiveComponent.SetMaterial` _sk_feetmesh _array_index _array_element))
  (return))

(fn `SetHandsMesh`
  (params (`Mesh Info` :type "/Game/LS_Template/Blueprints/Systems/Structures/Meshes/S_MeshInfo Structure"))
  (bind (_skeletalmesh _meshmaterials) (break `/Game/LS_Template/Blueprints/Systems/Structures/Meshes/S_MeshInfo` `Mesh Info`))
  (bind _sk_handsmesh (`self.SK_HandsMesh`))
  (`SkinnedMeshComponent.SetSkinnedAssetAndUpdate` _sk_handsmesh _skeletalmesh true)
  (for (_array_element _array_index) _meshmaterials
    (`PrimitiveComponent.SetMaterial` _sk_handsmesh _array_index _array_element))
  (return))

(fn `SetHeadMesh`
  (params (`Mesh Info` :type "/Game/LS_Template/Blueprints/Systems/Structures/Meshes/S_MeshInfo Structure"))
  (bind (_skeletalmesh _meshmaterials) (break `/Game/LS_Template/Blueprints/Systems/Structures/Meshes/S_MeshInfo` `Mesh Info`))
  (bind _mesh (`self.Mesh`))
  (`SkinnedMeshComponent.SetSkinnedAssetAndUpdate` _mesh _skeletalmesh true)
  (for (_array_element _array_index) _meshmaterials
    (`PrimitiveComponent.SetMaterial` _mesh _array_index _array_element))
  (return))

(fn `SetLegsMesh`
  (params (`Mesh Info` :type "/Game/LS_Template/Blueprints/Systems/Structures/Meshes/S_MeshInfo Structure"))
  (bind (_skeletalmesh _meshmaterials) (break `/Game/LS_Template/Blueprints/Systems/Structures/Meshes/S_MeshInfo` `Mesh Info`))
  (bind _sk_legsmesh (`self.SK_LegsMesh`))
  (`SkinnedMeshComponent.SetSkinnedAssetAndUpdate` _sk_legsmesh _skeletalmesh true)
  (for (_array_element _array_index) _meshmaterials
    (`PrimitiveComponent.SetMaterial` _sk_legsmesh _array_index _array_element))
  (return))

(fn `SetNPC_Mesh`
  (bind (_npc_info_npcrowname _npc_info_alreadyknownnpc_ _npc_info_npcname _npc_info_dialogdatatable _npc_info_charactermeshes) (break `/Game/LS_Template/Blueprints/Systems/Structures/NPC/S_NPC_Info` (`self.NPC_Info`)))
  (bind (_singlemesh _multipartmesh_ _hairmesh _headmesh _torsomesh _handsmesh _legsmesh _feetmesh) (break `/Game/LS_Template/Blueprints/Systems/Structures/Meshes/S_CharacterMesh` _npc_info_charactermeshes))
  (bind (_skeletalmesh _meshmaterials) (break `/Game/LS_Template/Blueprints/Systems/Structures/Meshes/S_MeshInfo` _singlemesh))
  (if _multipartmesh_
    ;[1 1 1] Sets each mesh parts and sets master pose
    (`self.SetHeadMesh` _headmesh)
    (`self.SetTorsoMesh` _torsomesh)
    (`self.SetHandsMesh` _handsmesh)
    (`self.SetLegsMesh` _legsmesh)
    (`self.SetFeetMesh` _feetmesh)
    (`SkinnedMeshComponent.SetLeaderPoseComponent` (`self.SK_TorsoMesh`) (`self.Mesh`) false)
    (`SkinnedMeshComponent.SetLeaderPoseComponent` (`self.SK_LegsMesh`) (`self.Mesh`) false)
    (`SkinnedMeshComponent.SetLeaderPoseComponent` (`self.SK_FeetMesh`) (`self.Mesh`) false)
    (`SkinnedMeshComponent.SetLeaderPoseComponent` (`self.SK_HandsMesh`) (`self.Mesh`) false)
    (return)
    (else
      ;[1 1 1] Sets the single mesh and destroys the unused skeletal meshes
      (`SkinnedMeshComponent.SetSkinnedAssetAndUpdate` (`self.Mesh`) _skeletalmesh true)
      (for (_array_element _array_index) _meshmaterials
        (`PrimitiveComponent.SetMaterial` (`self.Mesh`) _array_index _array_element))
      (`ActorComponent.K2_DestroyComponent` (`self.SK_TorsoMesh`))
      (`ActorComponent.K2_DestroyComponent` (`self.SK_LegsMesh`))
      (`ActorComponent.K2_DestroyComponent` (`self.SK_FeetMesh`))
      (`ActorComponent.K2_DestroyComponent` (`self.SK_HandsMesh`))
      (return))))

(fn `SetTorsoMesh`
  (params (`Mesh Info` :type "/Game/LS_Template/Blueprints/Systems/Structures/Meshes/S_MeshInfo Structure"))
  (bind (_skeletalmesh _meshmaterials) (break `/Game/LS_Template/Blueprints/Systems/Structures/Meshes/S_MeshInfo` `Mesh Info`))
  (bind _sk_torsomesh (`self.SK_TorsoMesh`))
  (`SkinnedMeshComponent.SetSkinnedAssetAndUpdate` _sk_torsomesh _skeletalmesh true)
  (for (_array_element _array_index) _meshmaterials
    (`PrimitiveComponent.SetMaterial` _sk_torsomesh _array_index _array_element))
  (return))

(fn `UserConstructionScript`
  (`parent.UserConstructionScript`)
  (bind _returnvalue (`|GetDataTableRow` "/Game/LS_Template/Blueprints/NPC/DT_NPC.DT_NPC" (`self.NPC_RowName`))
    (:`then`
      (set `self.NPC_Info` _returnvalue)
      (`self.SetNPC_Mesh`))))