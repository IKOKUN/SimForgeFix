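; BP_Item is a world pickup that adds a DT_Items entry to the player's inventory and destroys itself, or shows a HUD warning when no slot is free.
; The construction script applies the row's mesh and physics setting and configures a child BP_InteractionActor's shape and prompt location.
; That child actor's events trigger the pickup and, when outlines are enabled, toggle a custom-depth outline colored by rarity.
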(event `self.ReceiveBeginPlay`
  (bind (_iteminfos_itemrowname _iteminfos_itemname) (break `/Game/LS_Template/Blueprints/Systems/Structures/Items/S_ItemInfo` (`self.ItemInfos`)))
  (bind _interactionactor (`self.InteractionActor`))
  (`/Game/LS_Template/Blueprints/Interaction/Core/BP_InteractionActor.SetWidget` _interactionactor _iteminfos_itemname false 0 0)
  (add `/Game/LS_Template/Blueprints/Interaction/Core/BP_InteractionActor.OnInteraction` _interactionactor (delegate `OnInteractionEvent`))
  (add `/Game/LS_Template/Blueprints/Interaction/Core/BP_InteractionActor.OnSetUseable` _interactionactor (delegate `EventOnUseable`))
  (add `/Game/LS_Template/Blueprints/Interaction/Core/BP_InteractionActor.OnSetUnuseable` _interactionactor (delegate `EventOnUnuseable`)))

(event `OnInteractionEvent`
  (`self.ItemInteraction`))

(event `EventOnUseable`
  (`self.SetMeshOutline` true))

(event `EventOnUnuseable`
  (`self.SetMeshOutline` false))

(event `ItemInteraction`
  (bind _iteminfos_itemrowname (break `/Game/LS_Template/Blueprints/Systems/Structures/Items/S_ItemInfo` (`self.ItemInfos`)))
  ;[1 1 1] Event on Interaction
  (bind _success_ (`/Game/LS_Template/Blueprints/Systems/Core/BPL_Functions.SearchEmptySlot`))
  (if _success_
    (`/Game/LS_Template/Blueprints/Systems/Core/BPL_Functions.AddItemToInventory` _iteminfos_itemrowname (`self.ItemAmount`))
    (`self.K2_DestroyActor`)
    (else
      (`/Game/LS_Template/Blueprints/Systems/Core/BPL_Functions.DisplayHUD_Message` false "Your inventory is full !" (struct :`R` 0.994792 :`A` 1.0)))))

(fn `SetMeshOutline`
  (params (`Outline?` :type Boolean))
  (bind (_iteminfos_itemrowname _iteminfos_itemname _iteminfos_itemdescription _iteminfos_itemtype _iteminfos_clothestype _iteminfos_itemrarity) (break `/Game/LS_Template/Blueprints/Systems/Structures/Items/S_ItemInfo` (`self.ItemInfos`)))
  (if (`/Game/LS_Template/Blueprints/Systems/Core/LS_Instance.UseMeshOutline?` (`/Game/LS_Template/Blueprints/Systems/Core/BPL_Functions.Get_LST_Instance`))
    (`MaterialInstanceDynamic.SetVectorParameterValue` (`/Game/LS_Template/Blueprints/Interaction/Core/BPC_Interaction.OutlineDynamat` (`/Game/LS_Template/Blueprints/Systems/Core/Game/BP_LS_GameController.BPC_Interaction` (`/Game/LS_Template/Blueprints/Systems/Core/BPL_Functions.Get_LST_Controller`))) "OutlineColor" (select `/Game/LS_Template/Blueprints/Systems/Enumerations/Items/E_ItemRarity` _iteminfos_itemrarity :`NewEnumerator0` (struct :`R` 1.0 :`G` 1.0 :`B` 1.0 :`A` 1.0) :`NewEnumerator1` (struct :`R` 0.147275 :`G` 0.994792 :`B` 0.077031 :`A` 1.0) :`NewEnumerator2` (struct :`R` 0.034841 :`G` 0.438748 :`B` 1.0 :`A` 1.0) :`NewEnumerator3` (struct :`R` 0.247184 :`G` 0.108561 :`B` 0.90625 :`A` 1.0) :`NewEnumerator4` (struct :`R` 1.0 :`G` 0.573943 :`B` 0.003206 :`A` 1.0) :`NewEnumerator5` (struct :`R` 0.994792 :`A` 1.0) :!type "LinearColor Structure"))
    (`PrimitiveComponent.SetRenderCustomDepth` (`self.StaticMeshComponent`) `Outline?`)
    (return)
    (else
      (return))))

(fn `UserConstructionScript`
  (bind _interactionactor (`self.InteractionActor`))
  (bind _staticmeshcomponent (`self.StaticMeshComponent`))
  (bind _asbp_interaction_actor (cast `/Game/LS_Template/Blueprints/Interaction/Core/BP_InteractionActor` (`ChildActorComponent.ChildActor` (`self.ChildActor`))))
  (set `self.InteractionActor` _asbp_interaction_actor)
  (`/Game/LS_Template/Blueprints/Interaction/Core/BP_InteractionActor.HandleInteractionShape` _interactionactor (`self.InteractionShape`) (`self.SphereRadius`) (`self.BoxExtent`) (`self.CapsuleHalfHeight`) (`self.CapsuleRadius`))
  (`self.K2_SetActorRelativeLocation` _interactionactor (`self.InteractionLocation`) false false)
  (`SceneComponent.K2_SetRelativeLocation` (`/Game/LS_Template/Blueprints/Interaction/Core/BP_InteractionActor.Widget` _interactionactor) (`self.PromptLocation`) false false)
  (bind _returnvalue (`|GetDataTableRow` "/Game/LS_Template/Blueprints/Items/DT_Items.DT_Items" (`self.ItemRowName`))
    (:`then`
      (bind _output_get (set `self.ItemInfos` _returnvalue))
      (bind (_itemrowname _itemname _itemdescription _itemtype _clothestype _itemrarity _itemicon _itemsound _simulatephysics_ _itemmesh) (break `/Game/LS_Template/Blueprints/Systems/Structures/Items/S_ItemInfo` _output_get))
      (`StaticMeshComponent.SetStaticMesh` _staticmeshcomponent _itemmesh)
      (`PrimitiveComponent.SetSimulatePhysics` _staticmeshcomponent _simulatephysics_))))