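; Interactable door that can act as a shop entrance with opening hours and an optional item lock.
; A child BP_InteractionActor, configured in the construction script, drives interaction, prompt text and a color-coded mesh outline.
; Interaction checks days, holidays and hours, then consumes the required inventory item if locked, showing HUD messages on failure.
; Opening destroys the interaction actor and swings the mesh via timeline with collision disabled meanwhile, so it opens only once.
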(event `self.ReceiveBeginPlay`
  (bind _interactionactor (`self.InteractionActor`))
  (add `/Game/LS_Template/Blueprints/Interaction/Core/BP_InteractionActor.OnInteraction` _interactionactor (delegate `OnInteractionEvent`))
  (add `/Game/LS_Template/Blueprints/Interaction/Core/BP_InteractionActor.OnSetUseable` _interactionactor (delegate `EventOnUseable`))
  (add `/Game/LS_Template/Blueprints/Interaction/Core/BP_InteractionActor.OnSetUnuseable` _interactionactor (delegate `EventOnUnuseable`)))

(event `EventOnUseable`
  (`self.ProcessOutlineAndPromptText` true))

(event `EventOnUnuseable`
  (`self.ProcessOutlineAndPromptText` false))

(event `OnInteractionEvent`
  (`self.DoorInteraction`))

(event `DoorInteraction`
  (bind (_iteminfo_itemrowname _iteminfo_itemname _iteminfo_itemdescription _iteminfo_itemtype _iteminfo_clothestype _iteminfo_itemrarity _iteminfo_itemicon) (break `/Game/LS_Template/Blueprints/Systems/Structures/Items/S_ItemInfo` (`/Game/LS_Template/Blueprints/Systems/Core/BPL_Functions.GetItemInfoInDatatable` (`self.ItemRowName`))))
  ;[1 1 1] Is shop open ?
  (bind _opened_ (`self.IsDoorOpen?`))
  (if _opened_
    ;[1 1 1] Is door locked ?
    (if (`self.IsDoorLocked?`)
      ;[1 1 1] If true, checks if the inventory contains the item to unlocks it
      (bind (_itemfound_ _itemindex) (`/Game/LS_Template/Blueprints/Systems/Core/BPL_Functions.FindItemIndex` (`self.ItemRowName`)))
      (if _itemfound_
        ;[1 1 1] If true, removes the item from inventory
        (bind _success_ (`/Game/LS_Template/Blueprints/Systems/Core/BPL_Functions.RemoveItemFromInventory` _itemindex))
        (if _success_
          ;[1 1 1] Opens the door
          (`PrimitiveComponent.SetCollisionEnabled` (`self.SM_Door`) "NoCollision" :!label _label)
          (`PrimitiveComponent.SetCollisionEnabled` (`self.SM_GlassWindow`) "NoCollision")
          (`ActorComponent.K2_DestroyComponent` (`self.ChildActor`))
          (`self.SetMeshOutline` false)
          (bind (_direction _opendooralpha) (`Timeline|OpenDoorTL` :!via `PlayFromStart`)
            (:`Update`
              (`SceneComponent.K2_SetRelativeRotation` (`self.SM_Door`) (`KismetMathLibrary.RLerp` (struct) (struct :`Yaw` -90.0) _opendooralpha) false false))
            (:`Finished`
              (`PrimitiveComponent.SetCollisionEnabled` (`self.SM_Door`) "QueryOnly")
              (`PrimitiveComponent.SetCollisionEnabled` (`self.SM_GlassWindow`) "QueryOnly"))))
        (else
          ;[1 1 1] If false, displays an error message
          (`/Game/LS_Template/Blueprints/Systems/Core/BPL_Functions.DisplayHUD_Message` true (`|FormatText` "{ItemName} is needed to open this door" _iteminfo_itemname) (struct :`R` 0.994792 :`A` 1.0) _iteminfo_itemicon)
          (`/Game/LS_Template/Blueprints/Interaction/Core/BP_InteractionActor.HidePrompt` (`self.InteractionActor`) true)))
      (else
        (goto _label)))))

(fn `FormatOpeningMessage`
  (returns (OutMessage :type Text))
  (locals (LocalOpeningDaysString :type "Array of String") (LocalStringMessage :type String))
  (bind _localopeningdaysstring (`local.LocalOpeningDaysString`))
  (`KismetArrayLibrary.Array_Clear` (`local.LocalOpeningDaysString`))
  (for _array_element (`self.OpeningDays`)
    (`KismetArrayLibrary.Array_Add` (`local.LocalOpeningDaysString`) (`|GetEnumeratorNameAsString` _array_element)))
  (for (_array_element_2 _array_index) _localopeningdaysstring
    (set `local.LocalStringMessage` (`KismetStringLibrary.Concat_StrStr` (`local.LocalStringMessage`) _array_element_2))
    (if (< _array_index (- (`KismetArrayLibrary.Array_Length` _localopeningdaysstring) 1))
      (set `local.LocalStringMessage` (`KismetStringLibrary.Concat_StrStr` (`local.LocalStringMessage`) ", "))))
  (return (`|FormatText` "{ActivityName} is closed today. \nOpening Days : \n{Days}" (`self.ShopName`) (`KismetTextLibrary.Conv_StringToText` (`local.LocalStringMessage`)))))

(fn `IsDoorOpen?`
  (returns (`Opened?` :type Boolean))
  (locals (LocalCurrentDaytimeInt :type Integer))
  (bind (_currentday _daynumber _currentmonth _eventname _publicholiday_) (`/Game/LS_Template/Blueprints/Systems/Core/BPL_Functions.GetCurrentDate`))
  (bind _localcurrentdaytimeint (`local.LocalCurrentDaytimeInt`))
  ;[1 1 1] Is shop always opened ?
  (if (`self.IsAlwaysOpen?`)
    (return true)
    (else
      ;[1 1 1] Is Current day one of the opening days ?
      (if (`KismetArrayLibrary.Array_Contains` (`self.OpeningDays`) _currentday)
        ;[1 1 1] Is today a public holiday ?
        (if _publicholiday_
          (`/Game/LS_Template/Blueprints/Systems/Core/BPL_Functions.DisplayHUD_Message` false "Today is a public holiday" (struct :`R` 0.994792 :`A` 1.0))
          (return false)
          (else
            ;[1 1 1] Checks for Opening and closing time (the corresponding Int variables are set on the construction script)
            (set `local.LocalCurrentDaytimeInt` (`KismetMathLibrary.Conv_ByteToInt` (`/Game/LS_Template/Blueprints/Systems/Core/BPL_Functions.GetCurrentDaytime`)))
            (`/Engine/EditorBlueprintResources/StandardMacros.CompareInt` _localcurrentdaytimeint (`self.OpeningInt`)
              (:`>`
                (`/Engine/EditorBlueprintResources/StandardMacros.CompareInt` _localcurrentdaytimeint (`self.ClosingInt`) :!label _label
                  (:`>`
                    _)
                  (:`==`
                    _)
                  (:`<`
                    (return true))))
              (:`==`
                (goto _label))
              (:`<`
                _))
            (`/Game/LS_Template/Blueprints/Systems/Core/BPL_Functions.DisplayHUD_Message` false (`|FormatText` "{ActivityName} opens at {Openingtime} and closes at {ClosingTime}" (`self.ShopName`) (`KismetTextLibrary.Conv_StringToText` (`|GetEnumeratorNameAsString` (`self.OpeningTime`))) (`KismetTextLibrary.Conv_StringToText` (`|GetEnumeratorNameAsString` (`self.ClosingTime`)))) (struct :`R` 0.994792 :`A` 1.0))
            (return false)))
        (else
          (`/Game/LS_Template/Blueprints/Systems/Core/BPL_Functions.DisplayHUD_Message` false (`self.FormatOpeningMessage`) (struct :`R` 0.994792 :`A` 1.0))
          (return false))))))

(fn `ProcessOutlineAndPromptText`
  (params (`Outline?` :type Boolean))
  (if (`/Game/LS_Template/Blueprints/Systems/Core/LS_Instance.UseMeshOutline?` (`/Game/LS_Template/Blueprints/Systems/Core/BPL_Functions.Get_LST_Instance`))
    (`self.SetMeshOutline` `Outline?`))
  (bind _itemfound_ (`/Game/LS_Template/Blueprints/Systems/Core/BPL_Functions.FindItemIndex` (`self.ItemRowName`)))
  (`/Game/LS_Template/Blueprints/Interaction/Core/BP_InteractionActor.SetWidget` (`self.InteractionActor`) (select `bool` _itemfound_ :`false` "Locked" :`true` "Open" :!type "Text") false 0 0)
  (return))

(fn `SetMeshOutline`
  (params (`Outline?` :type Boolean))
  (locals (`LocalFound?` :type Boolean :default false))
  (bind _itemfound_ (`/Game/LS_Template/Blueprints/Systems/Core/BPL_Functions.FindItemIndex` (`self.ItemRowName`)))
  (set `local.LocalFound?` _itemfound_)
  (`MaterialInstanceDynamic.SetVectorParameterValue` (`/Game/LS_Template/Blueprints/Interaction/Core/BPC_Interaction.OutlineDynamat` (`/Game/LS_Template/Blueprints/Systems/Core/Game/BP_LS_GameController.BPC_Interaction` (`/Game/LS_Template/Blueprints/Systems/Core/BPL_Functions.Get_LST_Controller`))) "OutlineColor" (select `bool` (`self.IsDoorLocked?`) :`false` (struct :`R` 1.0 :`G` 1.0 :`B` 1.0 :`A` 1.0) :`true` (select `bool` (`local.LocalFound?`) :`false` (struct :`R` 0.994792 :`A` 1.0) :`true` (struct :`R` 0.147275 :`G` 0.994792 :`B` 0.077031 :`A` 1.0) :!type "LinearColor Structure")))
  (`PrimitiveComponent.SetRenderCustomDepth` (`self.SM_Door`) `Outline?`)
  (return))

(fn `UserConstructionScript`
  (bind _interactionactor (`self.InteractionActor`))
  (bind _asbp_interaction_actor (cast `/Game/LS_Template/Blueprints/Interaction/Core/BP_InteractionActor` (`ChildActorComponent.ChildActor` (`self.ChildActor`))))
  (set `self.InteractionActor` _asbp_interaction_actor)
  (`/Game/LS_Template/Blueprints/Interaction/Core/BP_InteractionActor.HandleInteractionShape` _interactionactor (`self.InteractionShape`) (`self.SphereRadius`) (`self.BoxExtent`) (`self.CapsuleHalfHeight`) (`self.CapsuleRadius`))
  (`self.K2_SetActorRelativeLocation` _interactionactor (`self.InteractionLocation`) false false)
  (`SceneComponent.K2_SetRelativeLocation` (`/Game/LS_Template/Blueprints/Interaction/Core/BP_InteractionActor.Widget` _interactionactor) (`self.PromptLocation`) false false)
  (set `self.OpeningInt` (`KismetMathLibrary.Conv_ByteToInt` (`self.OpeningTime`)))
  (set `self.ClosingInt` (`KismetMathLibrary.Conv_ByteToInt` (`self.ClosingTime`))))