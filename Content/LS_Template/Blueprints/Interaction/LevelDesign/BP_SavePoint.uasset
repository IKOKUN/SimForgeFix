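; BP_SavePoint is a level-placed interactable that saves the game, shows a HUD confirmation and hides its prompt.
; Its construction script configures a child BP_InteractionActor's shape, location and prompt position from the save point's variables.
; At BeginPlay it binds that actor's interaction, useable and unuseable events.
; Useable state toggles the prompt and, if the game instance enables it, a custom-depth mesh outline colored through the controller's outline material.
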(event `self.ReceiveBeginPlay`
  (bind _interactionactor (`self.InteractionActor`))
  (`/Game/LS_Template/Blueprints/Interaction/Core/BP_InteractionActor.SetWidget` _interactionactor "Save Game" false 0 0)
  (add `/Game/LS_Template/Blueprints/Interaction/Core/BP_InteractionActor.OnInteraction` _interactionactor (delegate `OnInteractionEvent`))
  (add `/Game/LS_Template/Blueprints/Interaction/Core/BP_InteractionActor.OnSetUseable` _interactionactor (delegate `EventOnUseable`))
  (add `/Game/LS_Template/Blueprints/Interaction/Core/BP_InteractionActor.OnSetUnuseable` _interactionactor (delegate `EventOnUnuseable`)))

(event `EventOnUnuseable`
  (`self.SetMeshOutline` false)
  (`/Game/LS_Template/Blueprints/Systems/Core/BPL_Functions.SetInteractTextWidget` "")
  (`/Game/LS_Template/Blueprints/Systems/Core/BPL_Functions.SetInteractWidgetVisibility` "Hidden"))

(event `OnInteractionEvent`
  (`/Game/LS_Template/Blueprints/Systems/Core/BPL_Functions.DisplayHUD_Message` true (`|FormatText` "{Message}" "Successfully Saving Game") (struct :`R` 1.0 :`G` 1.0 :`B` 1.0 :`A` 1.0) "/Game/LS_Template/Blueprints/UI/Textures/T_Save.T_Save")
  (`/Game/LS_Template/Blueprints/Systems/Core/BPL_Functions.SaveGame` false)
  (`/Game/LS_Template/Blueprints/Interaction/Core/BP_InteractionActor.HidePrompt` (`self.InteractionActor`) true))

(event `EventOnUseable`
  (`self.SetMeshOutline` true)
  (`/Game/LS_Template/Blueprints/Systems/Core/BPL_Functions.SetInteractTextWidget` "Save Game")
  (`/Game/LS_Template/Blueprints/Systems/Core/BPL_Functions.SetInteractWidgetVisibility` "SelfHitTestInvisible"))

(fn `SetMeshOutline`
  (params (`Outline?` :type Boolean))
  (if (`/Game/LS_Template/Blueprints/Systems/Core/LS_Instance.UseMeshOutline?` (`/Game/LS_Template/Blueprints/Systems/Core/BPL_Functions.Get_LST_Instance`))
    (`MaterialInstanceDynamic.SetVectorParameterValue` (`/Game/LS_Template/Blueprints/Interaction/Core/BPC_Interaction.OutlineDynamat` (`/Game/LS_Template/Blueprints/Systems/Core/Game/BP_LS_GameController.BPC_Interaction` (`/Game/LS_Template/Blueprints/Systems/Core/BPL_Functions.Get_LST_Controller`))) "OutlineColor" (`self.OutlineColor`))
    (`PrimitiveComponent.SetRenderCustomDepth` (`self.StaticMesh`) `Outline?`)
    (return)))

(fn `UserConstructionScript`
  (bind _interactionactor (`self.InteractionActor`))
  (bind _asbp_interaction_actor (cast `/Game/LS_Template/Blueprints/Interaction/Core/BP_InteractionActor` (`ChildActorComponent.ChildActor` (`self.ChildActor`))))
  (set `self.InteractionActor` _asbp_interaction_actor)
  (`/Game/LS_Template/Blueprints/Interaction/Core/BP_InteractionActor.HandleInteractionShape` _interactionactor (`self.InteractionShape`) (`self.SphereRadius`) (`self.BoxExtent`) (`self.CapsuleHalfHeight`) (`self.CapsuleRadius`))
  (`self.K2_SetActorRelativeLocation` _interactionactor (`self.InteractionLocation`) false false)
  (`SceneComponent.K2_SetRelativeLocation` (`/Game/LS_Template/Blueprints/Interaction/Core/BP_InteractionActor.Widget` _interactionactor) (`self.PromptLocation`) false false))