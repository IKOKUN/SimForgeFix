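; BP_Lift is an interactable level-design lift that moves its mesh between an original and a target location.
; A child BP_InteractionActor, configured in the construction script, supplies the shape and prompt and reports interaction and usability events.
; Each interaction alternately plays or reverses a timeline that lerps the mesh, with play rate derived from LiftTime.
; Usability toggles a custom-depth outline when the game instance enables it.
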(event `self.ReceiveBeginPlay`
  (bind _interactionactor (`self.InteractionActor`))
  (`/Game/LS_Template/Blueprints/Interaction/Core/BP_InteractionActor.SetWidget` _interactionactor "Lift" false 0 0)
  (add `/Game/LS_Template/Blueprints/Interaction/Core/BP_InteractionActor.OnInteraction` _interactionactor (delegate `OnInteractionEvent`))
  (add `/Game/LS_Template/Blueprints/Interaction/Core/BP_InteractionActor.OnSetUseable` _interactionactor (delegate `EventOnUseable`))
  (add `/Game/LS_Template/Blueprints/Interaction/Core/BP_InteractionActor.OnSetUnuseable` _interactionactor (delegate `EventOnUnuseable`)))

(event `EventOnUseable`
  (`self.SetMeshOutline` true))

(event `EventOnUnuseable`
  (`self.SetMeshOutline` false))

(event `OnInteractionEvent`
  (`self.UseLift`))

(event `UseLift`
  (`/Engine/EditorBlueprintResources/StandardMacros.FlipFlop`
    (:`A`
      (bind (_direction _liftalpha) (`Timeline|LiftTL` :!label _label)
        (:`Update`
          (`SceneComponent.K2_SetRelativeLocation` (`self.SM_Lift`) (`KismetMathLibrary.VLerp` (`self.OriginalLocation`) (`self.TargetLocation`) _liftalpha) false false))
        (:`Finished`
          (`/Game/LS_Template/Blueprints/Interaction/Core/BP_InteractionActor.HidePrompt` (`self.InteractionActor`) true))))
    (:`B`
      (goto _label :!via `Reverse`))))

(fn `SetMeshOutline`
  (params (`Outline?` :type Boolean))
  (if (`/Game/LS_Template/Blueprints/Systems/Core/LS_Instance.UseMeshOutline?` (`/Game/LS_Template/Blueprints/Systems/Core/BPL_Functions.Get_LST_Instance`))
    (`PrimitiveComponent.SetRenderCustomDepth` (`self.SM_Lift`) `Outline?`)
    (return)))

(fn `UserConstructionScript`
  (bind _interactionactor (`self.InteractionActor`))
  (bind _asbp_interaction_actor (cast `/Game/LS_Template/Blueprints/Interaction/Core/BP_InteractionActor` (`ChildActorComponent.ChildActor` (`self.ChildActor`))))
  (set `self.InteractionActor` _asbp_interaction_actor)
  (`/Game/LS_Template/Blueprints/Interaction/Core/BP_InteractionActor.HandleInteractionShape` _interactionactor (`self.InteractionShape`) (`self.SphereRadius`) (`self.BoxExtent`) (`self.CapsuleHalfHeight`) (`self.CapsuleRadius`))
  (`self.K2_SetActorRelativeLocation` _interactionactor (`self.InteractionLocation`) false false)
  (`SceneComponent.K2_SetRelativeLocation` (`/Game/LS_Template/Blueprints/Interaction/Core/BP_InteractionActor.Widget` _interactionactor) (`self.PromptLocation`) false false)
  (set `self.OriginalLocation` (`SceneComponent.RelativeLocation` (`self.SM_Lift`)))
  (`TimelineComponent.SetPlayRate` (`self.LiftTL`) (/ 1.0 (`self.LiftTime`))))