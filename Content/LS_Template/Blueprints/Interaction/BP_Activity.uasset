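; Placeable life-sim activity that the player uses, optionally with a known NPC, for energy and money to train stats.
; Interaction checks opening days, hours and holidays, then runs a timed, faded cutscene granting periodic experience from its stat list.
; A construction-built circular spline carries an orbiting camera, with tick enabled only during the cutscene.
; Afterwards it adjusts invited-NPC affection by tastes, optionally pays money and advances daytime.
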(event `self.ReceiveBeginPlay`
  (bind _interactionactor (`self.InteractionActor`))
  ;[1 1 1] Hide player mesh
  ; (Mesh needed to be visible to setup properly camera track so hide it here instead)
  (`SceneComponent.SetHiddenInGame` (`self.SK_PlayerMesh`) true true)
  (`/Game/LS_Template/Blueprints/Interaction/Core/BP_InteractionActor.SetWidget` _interactionactor (`self.ActivityName`) true (`self.MoneyCost`) (`KismetMathLibrary.FTrunc` (`self.EnergyCost`)))
  (add `/Game/LS_Template/Blueprints/Interaction/Core/BP_InteractionActor.OnInteraction` _interactionactor (delegate `OnInteractionEvent`))
  (add `/Game/LS_Template/Blueprints/Interaction/Core/BP_InteractionActor.OnSetUseable` _interactionactor (delegate `EventOnUseable`))
  (add `/Game/LS_Template/Blueprints/Interaction/Core/BP_InteractionActor.OnSetUnuseable` _interactionactor (delegate `EventOnUnuseable`))
  (bind _returnvalue (`|SpawnActorFromClass` "/Script/Engine.CameraActor" (`KismetMathLibrary.MakeTransform` (0.0 0.0 0.0)) "Undefined" "MultiplyWithRoot" null null))
  (set `self.CameraActor` _returnvalue)
  (`KismetSystemLibrary.Delay` 0.01)
  (`self.SetCustomMesh`))

(event `OnInteractionEvent`
  (bind _w_playerhud (`/Game/LS_Template/Blueprints/Systems/Core/BPL_Functions.Get_LST_PlayerHUD`))
  (`self.ActivityInteraction`)
  (if (`/Game/LS_Template/Blueprints/UI/W_PlayerHUD.IsStatsVisible` _w_playerhud)
    (`/Game/LS_Template/Blueprints/UI/W_PlayerHUD.DisplayHUD` _w_playerhud false false)
    (`/Game/LS_Template/Blueprints/Systems/Core/BPL_Functions.SetInteractTextWidget` "")
    (`/Game/LS_Template/Blueprints/Systems/Core/BPL_Functions.SetInteractWidgetVisibility` "Hidden")))

(event `EventOnUnuseable`
  (`self.SetMeshOutline` false)
  (`/Game/LS_Template/Blueprints/Systems/Core/BPL_Functions.SetInteractTextWidget` "")
  (`/Game/LS_Template/Blueprints/Systems/Core/BPL_Functions.SetInteractWidgetVisibility` "Hidden")
  (set `self.bHasInteract` false))

(event `EventOnUseable`
  (`self.SetMeshOutline` true)
  (if (not (`self.bHasInteract`))
    (`/Game/LS_Template/Blueprints/Systems/Core/BPL_Functions.SetInteractTextWidget` (`self.Interact Text`))
    (`/Game/LS_Template/Blueprints/Systems/Core/BPL_Functions.SetInteractWidgetVisibility` "SelfHitTestInvisible")
    (set `self.bHasInteract` true)))

(event `BeginExpTimer`
  ;[1 1 1] Timer experience
  (bind _returnvalue (`KismetSystemLibrary.K2_SetTimerDelegate` (delegate `GainExp`) 1.0 true)))

(event `StopTimerExperience`
  ;[1 1 1] Timer experience
  (`KismetSystemLibrary.K2_ClearAndInvalidateTimerHandle` (stale `BeginExpTimer` _returnvalue)))

(event `GainExp`
  (bind _activitystat (`self.ActivityStat`))
  ;[1 1 1] Gain experience based on chosen stats
  (`/Game/LS_Template/Blueprints/Systems/Core/BPL_Functions.GainStatExperience` (`|GetArrayItem` _activitystat (`KismetMathLibrary.RandomIntegerInRange` 0 (`KismetArrayLibrary.Array_LastIndex` _activitystat))) (select `bool` (`self.GainFixedAmount?`) :`false` (`KismetMathLibrary.RandomFloatInRange` (`self.MinimumGain`) (`self.MaximumGain`)) :`true` (`self.FixedAmountToGain`))))

(event `self.ReceiveTick`
  (params (DeltaSeconds :type "Float (single-precision)"))
  ;[1 1 1] Event tick - To smoothly moves the camera - This actor only ticks when needed, see function "Start Ticking Event"
  (if (`self.MoveCamera?`)
    (if (>= (`self.PathDistance`) (`SplineComponent.GetSplineLength` (`self.CameraSpline`)))
      (set `self.PathDistance` 0.0))
    (bind _output_get (set `self.PathDistance` (+ (`self.PathDistance`) (* (`self.Speed`) (`GameplayStatics.GetWorldDeltaSeconds`)))))
    (`self.UpdateCameraLocAndRot` _output_get)))

(event `ActivityInteraction`
  (bind _opened_ (`self.IsActivityOpen?`))
  (if _opened_
    (if (`self.CanInviteNPC?`)
      (`self.DisplayInvitationWidget`)
      (else
        (`self.StartActivity` false)))
    (`/Game/LS_Template/Blueprints/Systems/Core/BPL_Functions.SetInteractTextWidget` "")
    (`/Game/LS_Template/Blueprints/Systems/Core/BPL_Functions.SetInteractWidgetVisibility` "Hidden")))

(event `StartActivity`
  (params (`NPC_Invited?` :type Boolean) (Invited_NPC_RowName :type Name))
  (bind _invitedstorynpc (`self.InvitedStoryNPC`))
  ;[1 1 1] Checks if the activity is open, if the player have enough energy and money
  (set `self.NPC_Invited?` `NPC_Invited?`)
  (set `self.InvitedNPC_RowName` Invited_NPC_RowName)
  (bind _success_ (`/Game/LS_Template/Blueprints/Systems/Core/BPL_Functions.RemoveEnergy` (`self.EnergyCost`)))
  (if _success_
    (bind _success__2 (`/Game/LS_Template/Blueprints/Systems/Core/BPL_Functions.RemoveMoney` (`self.MoneyCost`)))
    (if _success__2
      ;[1 1 1] Select a random point on the camera track
      (set `self.PathDistance` (`KismetMathLibrary.RandomFloatInRange` 0.0 1450.0))
      ;[1 1 1] Before Activity
      (`self.HandleInputs` true)
      (`/Game/LS_Template/Blueprints/Systems/Core/BPL_Functions.CameraFadeOut` 1.0)
      (`KismetSystemLibrary.Delay` 1.0)
      (`self.StartTickingEvent` true)
      (`self.BlendView` true)
      (`self.SetActivityMesh` true)
      (`/Game/LS_Template/Blueprints/Systems/Core/BPL_Functions.CameraFadeIn` 1.0)
      (`KismetSystemLibrary.Delay` 1.0)
      ;[1 1 1] During Activity
      (`self.GainExp`)
      (`self.BeginExpTimer`)
      (`KismetSystemLibrary.Delay` 5.0)
      (`self.StopTimerExperience`)
      (`KismetSystemLibrary.Delay` 1.0)
      ;[1 1 1] After Activity
      (`/Game/LS_Template/Blueprints/Systems/Core/BPL_Functions.CameraFadeOut` 1.0)
      (`KismetSystemLibrary.Delay` 1.0)
      (`self.BlendView` false)
      (`self.SetActivityMesh` false)
      (`self.StartTickingEvent` false)
      (`/Game/LS_Template/Blueprints/Systems/Core/BPL_Functions.CameraFadeIn` 1.0)
      (`self.HandleInputs` false)
      (if (`self.NPC_Invited?`)
        (`self.ProcessAffectionGain`))
      (`/Game/LS_Template/Blueprints/Interaction/Core/BP_InteractionActor.HidePrompt` (`self.InteractionActor`) true)
      (if (`self.GainMoney?`)
        (`/Game/LS_Template/Blueprints/Systems/Core/BPL_Functions.AddMoney` (`self.MoneyGain`)))
      (`KismetSystemLibrary.Delay` 1.0)
      (`/Game/LS_Template/Blueprints/Systems/Core/BPL_Functions.AdvanceDayTime` false)
      (`/Game/LS_Template/Blueprints/Interaction/Core/BP_InteractionActor.HidePrompt` (`self.InteractionActor`) true)
      (set `self.W_NPC_Invitation` null)
      (`/Engine/EditorBlueprintResources/StandardMacros.IsValid` _invitedstorynpc
        (:`Is Valid`
          (`self.SetActorHiddenInGame` _invitedstorynpc false)
          (set `self.InvitedStoryNPC` null))
        (:`Is Not Valid`
          _))
      (set `self.bHasInteract` false)
      (`/Game/LS_Template/Blueprints/Systems/Core/BPL_Functions.SetInteractTextWidget` (`self.Interact Text`))
      (`/Game/LS_Template/Blueprints/Systems/Core/BPL_Functions.SetInteractWidgetVisibility` "SelfHitTestInvisible")
      (else
        (`/Game/LS_Template/Blueprints/Interaction/Core/BP_InteractionActor.HidePrompt` (`self.InteractionActor`) true :!label _label)))
    (else
      (goto _label))))

(fn `BlendView`
  (params (`BlendIn?` :type Boolean))
  (bind _lst_controller (`/Game/LS_Template/Blueprints/Systems/Core/BPL_Functions.Get_LST_Controller`))
  (if `BlendIn?`
    (`PlayerController.SetViewTargetWithBlend` _lst_controller (`self.CameraActor`) 0.0 "VTBlend_Linear" 0.0 false)
    (else
      (`PlayerController.SetViewTargetWithBlend` _lst_controller (`GameplayStatics.GetPlayerCharacter` 0) 0.0 "VTBlend_Linear" 0.0 false))))

(fn `DisplayInvitationWidget`
  (bind _lst_controller (`/Game/LS_Template/Blueprints/Systems/Core/BPL_Functions.Get_LST_Controller`))
  (bind _w_playerhud (`/Game/LS_Template/Blueprints/Systems/Core/BPL_Functions.Get_LST_PlayerHUD`))
  (if (> (`KismetArrayLibrary.Array_Length` (`/Game/LS_Template/Blueprints/Systems/Core/LS_Instance.KnownsNPC` (`/Game/LS_Template/Blueprints/Systems/Core/BPL_Functions.Get_LST_Instance`))) 0)
    (`/Engine/EditorBlueprintResources/StandardMacros.IsValid` (`self.W_NPC_Invitation`)
      (:`Is Valid`
        _)
      (:`Is Not Valid`
        (bind _returnvalue (`|CreateWidget` "/Game/LS_Template/Blueprints/UI/Activity/W_NPC_Invitation.W_NPC_Invitation_C" null self))
        (set `self.W_NPC_Invitation` _returnvalue)))
    (`UserWidget.AddToViewport` (`self.W_NPC_Invitation`) 0)
    (if (`/Game/LS_Template/Blueprints/UI/W_PlayerHUD.IsStatsVisible` _w_playerhud)
      (`/Game/LS_Template/Blueprints/UI/W_PlayerHUD.DisplayHUD` _w_playerhud false false))
    (set `PlayerController.bShowMouseCursor` true _lst_controller)
    (`WidgetBlueprintLibrary.SetInputMode_UIOnlyEx` _lst_controller (`self.W_NPC_Invitation`))
    (return)
    (else
      (`self.StartActivity` false)
      (return))))

(fn `DoesNPC_LikedActivity?`
  (returns (`Liked?` :type Boolean))
  (locals (LocalLikeInt :type Integer) (LocalDislikeInt :type Integer))
  (bind (_likedactivities _dislikedactivities) (break `/Game/LS_Template/Blueprints/Systems/Structures/NPC/S_NPC_Tastes` (`.NPCTastes_65_F0065F5E45BA216293BA999CAD516BD3` (break `/Game/LS_Template/Blueprints/Systems/Structures/NPC/S_NPC_Info` (`self.NPC_Infos`)))))
  (for _array_element _likedactivities
    (if (`KismetArrayLibrary.Array_Contains` (`self.ActivityStat`) _array_element)
      (`/Engine/EditorBlueprintResources/StandardMacros.IncrementInt` (`local.LocalLikeInt`))))
  (for _array_element_2 _dislikedactivities
    (if (`KismetArrayLibrary.Array_Contains` (`self.ActivityStat`) _array_element_2)
      (`/Engine/EditorBlueprintResources/StandardMacros.IncrementInt` (`local.LocalDislikeInt`))))
  (return (> (`local.LocalLikeInt`) (`local.LocalDislikeInt`))))

(fn `DoesPlayerKnowNPC?`
  (returns (ReturnValue :type Boolean))
  (return (> (`KismetArrayLibrary.Array_Length` (`/Game/LS_Template/Blueprints/Systems/Core/LS_Instance.KnownsNPC` (`/Game/LS_Template/Blueprints/Systems/Core/BPL_Functions.Get_LST_Instance`))) 0)))

(fn `FindAndHideStoryNPC`
  (bind _invitedstorynpc (`self.InvitedStoryNPC`))
  (bind _outactors (`GameplayStatics.GetAllActorsOfClass` "/Game/LS_Template/Blueprints/NPC/BPC_NPC_Story.BPC_NPC_Story_C"))
  (for _array_element _outactors
    (bind _npc_info_npcrowname (break `/Game/LS_Template/Blueprints/Systems/Structures/NPC/S_NPC_Info` (`/Game/LS_Template/Blueprints/NPC/BPC_NPC_Story.NPC_Info` _array_element)))
    (if (== _npc_info_npcrowname (`self.InvitedNPC_RowName`))
      (set `self.InvitedStoryNPC` _array_element)
      (break)))
  (`/Engine/EditorBlueprintResources/StandardMacros.IsValid` _invitedstorynpc
    (:`Is Valid`
      (`self.SetActorHiddenInGame` _invitedstorynpc true))
    (:`Is Not Valid`
      _))
  (return))

(fn `FormatOpeningDaysMessage`
  (returns (OutMessage :type Text))
  (locals (LocalOpeningDaysString :type "Array of String") (LocalStringMessage :type String))
  (bind _localopeningdaysstring (`local.LocalOpeningDaysString`))
  (`KismetArrayLibrary.Array_Clear` (`local.LocalOpeningDaysString`))
  (for _array_element (`self.OpeningDays`)
    (`KismetArrayLibrary.Array_Add` (`local.LocalOpeningDaysString`) (`|GetEnumeratorNameAsString` _array_element)))
  (for (_array_element_2 _array_index) _localopeningdaysstring
    (set `local.LocalStringMessage` (`KismetStringLibrary.Concat_StrStr` (`local.LocalStringMessage`) _array_element_2))
    (if (< _array_index (- (`KismetArrayLibrary.Array_Length` _localopeningdaysstring) 1))
      (set `local.LocalStringMessage` (`KismetStringLibrary.Concat_StrStr` (`local.LocalStringMessage`) ", "))))
  (return (`|FormatText` "{ActivityName} is closed today. \nOpening Days : \n{Days}" (`self.ActivityName`) (`KismetTextLibrary.Conv_StringToText` (`local.LocalStringMessage`)))))

(fn `GetPathLocationAtDistance`
  (params (Time :type "Float (double-precision)"))
  (returns (WorldLocation :type "Vector Structure"))
  (return (`SplineComponent.GetLocationAtDistanceAlongSpline` (`self.CameraSpline`) Time "World")))

(fn `HandleInputs`
  (params (`DisableInputs?` :type Boolean))
  (bind _lst_controller (`/Game/LS_Template/Blueprints/Systems/Core/BPL_Functions.Get_LST_Controller`))
  (bind _returnvalue (`GameplayStatics.GetPlayerCharacter` 0))
  (if `DisableInputs?`
    (`self.DisableInput` _returnvalue _lst_controller)
    (`self.DisableInput` _lst_controller _lst_controller)
    (return)
    (else
      (`self.EnableInput` _returnvalue _lst_controller)
      (`self.EnableInput` _lst_controller _lst_controller)
      (return))))

(fn `IsActivityOpen?`
  (returns (`Opened?` :type Boolean))
  (locals (LocalCurrentDaytimeInt :type Integer :default 0))
  (bind (_currentday _daynumber _currentmonth _eventname _publicholiday_) (`/Game/LS_Template/Blueprints/Systems/Core/BPL_Functions.GetCurrentDate`))
  (bind _localcurrentdaytimeint (`local.LocalCurrentDaytimeInt`))
  ;[1 1 1] Is Activity always opened ?
  (if (`self.IsAlwaysOpen?`)
    (return true)
    (else
      ;[1 1 1] Is Current day one of the opening days ?
      (if (`KismetArrayLibrary.Array_Contains` (`self.OpeningDays`) _currentday)
        ;[1 1 1] Is today a public holiday ?
        (if _publicholiday_
          (`/Game/LS_Template/Blueprints/Systems/Core/BPL_Functions.DisplayHUD_Message` false "Today is a public holiday" (struct :`R` 0.994792 :`A` 1.0))
          (return false)
          (else
            ;[1 1 1] Checks for Opening and closing time (the corresponding Int variables are set on the construction script)
            (set `local.LocalCurrentDaytimeInt` (`KismetMathLibrary.Conv_ByteToInt` (`/Game/LS_Template/Blueprints/Systems/Core/BPL_Functions.GetCurrentDaytime`)))
            (`/Engine/EditorBlueprintResources/StandardMacros.CompareInt` _localcurrentdaytimeint (`self.OpeningInt`)
              (:`>`
                (`/Engine/EditorBlueprintResources/StandardMacros.CompareInt` _localcurrentdaytimeint (`self.ClosingInt`) :!label _label
                  (:`>`
                    _)
                  (:`==`
                    _)
                  (:`<`
                    (return true))))
              (:`==`
                (goto _label))
              (:`<`
                _))
            (`/Game/LS_Template/Blueprints/Systems/Core/BPL_Functions.DisplayHUD_Message` false (`|FormatText` "{ActivityName} opens at {Openingtime} and closes at {ClosingTime}" (`self.ActivityName`) (`KismetTextLibrary.Conv_StringToText` (`|GetEnumeratorNameAsString` (`self.OpeningTime`))) (`KismetTextLibrary.Conv_StringToText` (`|GetEnumeratorNameAsString` (`self.ClosingTime`)))) (struct :`R` 0.994792 :`A` 1.0))
            (return false)))
        (else
          (`/Game/LS_Template/Blueprints/Systems/Core/BPL_Functions.DisplayHUD_Message` false (`self.FormatOpeningDaysMessage`) (struct :`R` 0.994792 :`A` 1.0))
          (return false))))))

(fn `ProcessAffectionGain`
  (locals (`LocalLiked?` :type Boolean :default false))
  (bind _affectionamount (`self.AffectionAmount`))
  (bind _localliked_ (`local.LocalLiked?`))
  (bind _invitednpc_rowname (`self.InvitedNPC_RowName`))
  (bind _returnvalue (`KismetTextLibrary.Conv_DoubleToText` (`self.AffectionAmount`) "HalfToEven" false true 1 324 0 0))
  (bind (_success_ _npc_info) (`/Game/LS_Template/Blueprints/Systems/Core/BPL_Functions.GetNPC_Info` (`self.InvitedNPC_RowName`)))
  (bind _output_get (set `local.LocalLiked?` (`self.DoesNPC_LikedActivity?`)))
  (if _output_get
    (`/Game/LS_Template/Blueprints/Systems/Core/BPL_Functions.AddAffection` _invitednpc_rowname _affectionamount)
    (else
      (`/Game/LS_Template/Blueprints/Systems/Core/BPL_Functions.RemoveAffection` _invitednpc_rowname _affectionamount)))
  (`/Game/LS_Template/Blueprints/Systems/Core/BPL_Functions.DisplayHUD_Message` true (select `bool` _localliked_ :`false` (`|FormatText` "{NPC_Name} got bored \nYou lost {AffectionAmount} affection with her !" (`.NPCName_28_C5B09B6449FFD0C04B1F848EED4FF3D5` (break `/Game/LS_Template/Blueprints/Systems/Structures/NPC/S_NPC_Info` _npc_info)) _returnvalue) :`true` (`|FormatText` "{NPC_Name} had fun \nYou gain {AffectionAmount} affection with her !" (`.NPCName_28_C5B09B6449FFD0C04B1F848EED4FF3D5` (break `/Game/LS_Template/Blueprints/Systems/Structures/NPC/S_NPC_Info` _npc_info)) _returnvalue)) (select `bool` _localliked_ :`false` (struct :`R` 1.0 :`A` 1.0) :`true` (struct :`R` 0.303662 :`G` 0.96875 :`B` 0.148631 :`A` 1.0) :!type "LinearColor Structure") "/Engine/EngineResources/AICON-Green.AICON-Green")
  (return))

(fn `SetActivityMesh`
  (params (`Beginning?` :type Boolean))
  (locals (`LocalBegin?` :type Boolean))
  (bind _sk_npc_mesh (`self.SK_NPC_Mesh`))
  (set `local.LocalBegin?` `Beginning?`)
  ;[0.9948 0 0] Cast to your own character here
  (bind _asthird_person_character (cast `/Game/LS_Template/EpicContent/CharacterExampleContent/ThirdPersonCharacter` (`GameplayStatics.GetPlayerCharacter` 0)))
  (`SkeletalMeshComponent.PlayAnimation` (`self.SK_PlayerMesh`) (`self.AnimationToPlay`) true)
  (if (`self.NPC_Invited?`)
    (`self.SetNPC_Mesh`)
    (`SceneComponent.SetHiddenInGame` _sk_npc_mesh (not (`local.LocalBegin?`)) true)
    (`SkeletalMeshComponent.PlayAnimation` _sk_npc_mesh (`self.AnimationToPlay`) true)
    (`self.FindAndHideStoryNPC`)
    (return)
    (else
      (return))))

(fn `SetCustomMesh`
  (bind _sk_playermesh (`self.SK_PlayerMesh`))
  (bind _sk_playermesh_2 (`self.SK_PlayerMesh`))
  (bind _sk_feetmesh (`self.SK_FeetMesh`))
  (bind _sk_hairmesh (`self.SK_HairMesh`))
  (bind _sk_torsomesh (`self.SK_TorsoMesh`))
  (bind _sk_handsmesh (`self.SK_HandsMesh`))
  (bind _sk_legsmesh (`self.SK_LegsMesh`))
  (bind (_singlemesh _multipartmesh_ _hairmesh _headmesh _torsomesh _handsmesh _legsmesh _feetmesh) (break `/Game/LS_Template/Blueprints/Systems/Structures/Meshes/S_CharacterMesh` (`.CharacterMeshes` (`/Game/LS_Template/Blueprints/Systems/Core/BPL_Functions.GetPlayerInfo`))))
  (bind (_skeletalmesh _meshmaterials) (break `/Game/LS_Template/Blueprints/Systems/Structures/Meshes/S_MeshInfo` _feetmesh))
  (bind (_skeletalmesh_2 _meshmaterials_2) (break `/Game/LS_Template/Blueprints/Systems/Structures/Meshes/S_MeshInfo` _headmesh))
  (bind (_skeletalmesh_3 _meshmaterials_3) (break `/Game/LS_Template/Blueprints/Systems/Structures/Meshes/S_MeshInfo` _singlemesh))
  (bind (_skeletalmesh_4 _meshmaterials_4) (break `/Game/LS_Template/Blueprints/Systems/Structures/Meshes/S_MeshInfo` _hairmesh))
  (bind (_skeletalmesh_5 _meshmaterials_5) (break `/Game/LS_Template/Blueprints/Systems/Structures/Meshes/S_MeshInfo` _torsomesh))
  (bind (_skeletalmesh_6 _meshmaterials_6) (break `/Game/LS_Template/Blueprints/Systems/Structures/Meshes/S_MeshInfo` _handsmesh))
  (bind (_skeletalmesh_7 _meshmaterials_7) (break `/Game/LS_Template/Blueprints/Systems/Structures/Meshes/S_MeshInfo` _legsmesh))
  (if _multipartmesh_
    ;[1 1 1] Head Mesh (used as master pose)
    (`SkinnedMeshComponent.SetSkinnedAssetAndUpdate` _sk_playermesh _skeletalmesh_2 true)
    (for (_array_element _array_index) _meshmaterials_2
      (`PrimitiveComponent.SetMaterial` _sk_playermesh _array_index _array_element))
    ;[1 1 1] Hair Mesh
    (`SkinnedMeshComponent.SetSkinnedAssetAndUpdate` _sk_hairmesh _skeletalmesh_4 true)
    (for (_array_element_2 _array_index_2) _meshmaterials_4
      (`PrimitiveComponent.SetMaterial` _sk_hairmesh _array_index_2 _array_element_2))
    ;[1 1 1] TorsoMesh
    (`SkinnedMeshComponent.SetSkinnedAssetAndUpdate` _sk_torsomesh _skeletalmesh_5 true)
    (for (_array_element_3 _array_index_3) _meshmaterials_5
      (`PrimitiveComponent.SetMaterial` _sk_torsomesh _array_index_3 _array_element_3))
    ;[1 1 1] Hands Mesh
    (`SkinnedMeshComponent.SetSkinnedAssetAndUpdate` _sk_handsmesh _skeletalmesh_6 true)
    (for (_array_element_4 _array_index_4) _meshmaterials_6
      (`PrimitiveComponent.SetMaterial` _sk_handsmesh _array_index_4 _array_element_4))
    ;[1 1 1] Legs Mesh
    (`SkinnedMeshComponent.SetSkinnedAssetAndUpdate` _sk_legsmesh _skeletalmesh_7 true)
    (for (_array_element_5 _array_index_5) _meshmaterials_7
      (`PrimitiveComponent.SetMaterial` _sk_legsmesh _array_index_5 _array_element_5))
    ;[1 1 1] Feet Mesh
    (`SkinnedMeshComponent.SetSkinnedAssetAndUpdate` _sk_feetmesh _skeletalmesh true)
    (for (_array_element_6 _array_index_6) _meshmaterials
      (`PrimitiveComponent.SetMaterial` _sk_feetmesh _array_index_6 _array_element_6))
    (`SkinnedMeshComponent.SetLeaderPoseComponent` (`self.SK_HandsMesh`) (`self.SK_PlayerMesh`) false false)
    (`SkinnedMeshComponent.SetLeaderPoseComponent` (`self.SK_LegsMesh`) (`self.SK_PlayerMesh`) false false)
    (`SkinnedMeshComponent.SetLeaderPoseComponent` (`self.SK_FeetMesh`) (`self.SK_PlayerMesh`) false false)
    (`SkinnedMeshComponent.SetLeaderPoseComponent` (`self.SK_HairMesh`) (`self.SK_PlayerMesh`) false false)
    (`SkinnedMeshComponent.SetLeaderPoseComponent` (`self.SK_TorsoMesh`) (`self.SK_PlayerMesh`) false false)
    (return)
    (else
      (`SkinnedMeshComponent.SetSkinnedAssetAndUpdate` _sk_playermesh_2 _skeletalmesh_3 true)
      (for (_array_element_7 _array_index_7) _meshmaterials_3
        (`PrimitiveComponent.SetMaterial` _sk_playermesh_2 _array_index_7 _array_element_7))
      (`ActorComponent.K2_DestroyComponent` (`self.SK_HairMesh`))
      (`ActorComponent.K2_DestroyComponent` (`self.SK_TorsoMesh`))
      (`ActorComponent.K2_DestroyComponent` (`self.SK_HandsMesh`))
      (`ActorComponent.K2_DestroyComponent` (`self.SK_LegsMesh`))
      (`ActorComponent.K2_DestroyComponent` (`self.SK_FeetMesh`))
      (return))))

(fn `SetMeshOutline`
  (params (`Outline?` :type Boolean))
  (if (`/Game/LS_Template/Blueprints/Systems/Core/LS_Instance.UseMeshOutline?` (`/Game/LS_Template/Blueprints/Systems/Core/BPL_Functions.Get_LST_Instance`))
    (`MaterialInstanceDynamic.SetVectorParameterValue` (`/Game/LS_Template/Blueprints/Interaction/Core/BPC_Interaction.OutlineDynamat` (`/Game/LS_Template/Blueprints/Systems/Core/Game/BP_LS_GameController.BPC_Interaction` (`/Game/LS_Template/Blueprints/Systems/Core/BPL_Functions.Get_LST_Controller`))) "OutlineColor" (`self.OutlineColor`))
    (`PrimitiveComponent.SetRenderCustomDepth` (`self.SM_ActivityMesh`) `Outline?`)
    (return)))

(fn `SetNPC_Mesh`
  (bind _sk_npc_mesh (`self.SK_NPC_Mesh`))
  (bind (_success_ _npc_info) (`/Game/LS_Template/Blueprints/Systems/Core/BPL_Functions.GetNPC_Info` (`self.InvitedNPC_RowName`)))
  (bind _output_get (set `self.NPC_Infos` _npc_info))
  (if _success_
    (bind (_singlemesh _multipartmesh_) (break `/Game/LS_Template/Blueprints/Systems/Structures/Meshes/S_CharacterMesh` (`.CharacterMeshes_56_27EDF5F140DD3B35F63D9C9FAC29B660` (break `/Game/LS_Template/Blueprints/Systems/Structures/NPC/S_NPC_Info` _output_get))))
    (if (not _multipartmesh_)
      (bind (_skeletalmesh _meshmaterials) (break `/Game/LS_Template/Blueprints/Systems/Structures/Meshes/S_MeshInfo` _singlemesh))
      (`SkinnedMeshComponent.SetSkinnedAssetAndUpdate` _sk_npc_mesh _skeletalmesh true)
      (for (_array_element _array_index) _meshmaterials
        (`PrimitiveComponent.SetMaterial` _sk_npc_mesh _array_index _array_element))
      (return))
    (else
      (`KismetSystemLibrary.PrintString` "Can't retrieve NPC_RowName in NPC_Datable \nError coming from \"Set NPC_Mesh\" in BP_Activity\"")
      (return))))

(fn `StartTickingEvent`
  (params (`MoveCamera?` :type Boolean))
  (bind _output_get (set `self.MoveCamera?` `MoveCamera?`))
  (`self.SetActorTickEnabled` _output_get)
  (return))

(fn `UpdateCameraLocAndRot`
  (params (Time :type "Float (double-precision)"))
  (bind _cameraactor (`self.CameraActor`))
  (`self.K2_SetActorLocation` _cameraactor (`self.GetPathLocationAtDistance` Time) false false)
  (`self.K2_SetActorRotation` _cameraactor (`KismetMathLibrary.FindLookAtRotation` (`self.K2_GetActorLocation` _cameraactor) (+ (`self.K2_GetActorLocation`) (`self.CameraFocusPoint`))) false)
  (return))

(fn `UserConstructionScript`
  (bind _sk_playermesh (`self.SK_PlayerMesh`))
  (bind _sk_npc_mesh (`self.SK_NPC_Mesh`))
  (bind _radius (`self.Radius`))
  (bind _previewcamera (`self.PreviewCamera`))
  (bind _cameraspline (`self.CameraSpline`))
  (bind _sm_activitymesh (`self.SM_ActivityMesh`))
  (bind _singleanimationplaydata (make `SingleAnimationPlayData` (`self.AnimationToPlay`)))
  (bind _asbp_interaction_actor (cast `/Game/LS_Template/Blueprints/Interaction/Core/BP_InteractionActor` (`ChildActorComponent.ChildActor` (`self.ChildActor`))))
  (bind _output_get (set `self.InteractionActor` _asbp_interaction_actor))
  (`/Game/LS_Template/Blueprints/Interaction/Core/BP_InteractionActor.HandleInteractionShape` _output_get (`self.InteractionShape`) (`self.SphereRadius`) (`self.BoxExtent`) (`self.CapsuleHalfHeight`) (`self.CapsuleRadius`))
  (`self.K2_SetActorRelativeLocation` _output_get (`self.InteractionLocation`) false false)
  (`SceneComponent.K2_SetRelativeLocation` (`/Game/LS_Template/Blueprints/Interaction/Core/BP_InteractionActor.Widget` _output_get) (`self.PromptLocation`) false false)
  (`StaticMeshComponent.SetStaticMesh` _sm_activitymesh (`self.ActivityMesh`))
  (`SceneComponent.SetRelativeScale3D` _sm_activitymesh (`self.MeshScale`))
  (`SceneComponent.K2_SetRelativeLocation` _sk_playermesh (`self.PlayerMeshLocation`) false false)
  (`SceneComponent.K2_SetRelativeRotation` _sk_playermesh (`self.PlayerMeshRotation`) false false)
  (`SceneComponent.K2_SetRelativeLocation` _sk_npc_mesh (`self.NPC_MeshLocation`) false false)
  (`SceneComponent.K2_SetRelativeRotation` _sk_npc_mesh (`self.NPC_MeshRotation`) false false)
  (`SceneComponent.K2_SetRelativeLocation` (`self.CameraSpline`) (`self.TrackLocation`) false false)
  (set `SkeletalMeshComponent.AnimationData` _singleanimationplaydata (`self.SK_PlayerMesh`))
  (set `SkeletalMeshComponent.AnimationData` _singleanimationplaydata (`self.SK_NPC_Mesh`))
  (set `self.OpeningInt` (`KismetMathLibrary.Conv_ByteToInt` (`self.OpeningTime`)))
  (set `self.ClosingInt` (`KismetMathLibrary.Conv_ByteToInt` (`self.ClosingTime`)))
  (set `self.PreviewTime` (`KismetMathLibrary.FClamp` (`self.PreviewTime`)))
  (`|ExecutionSequence`
    (:`then_0`
      (`SplineComponent.SetClosedLoop` _cameraspline true true)
      (`SplineComponent.ClearSplinePoints` _cameraspline true)
      (for _index (range 1 (+ (`self.SplinePointsAmount`) 1))
        (bind _returnvalue (* _index (/ 360.0 (`KismetMathLibrary.Conv_IntToDouble` (`self.SplinePointsAmount`)))))
        (`SplineComponent.AddSplinePoint` (`self.CameraSpline`) (`KismetMathLibrary.MakeVector` (* _radius (`KismetMathLibrary.DegCos` _returnvalue)) (* _radius (`KismetMathLibrary.DegSin` _returnvalue))) "Local" true)))
    (:`then_1`
      (`SceneComponent.K2_SetRelativeRotation` :`self` (`self.CameraSpline`)))
    (:`then_2`
      (`SceneComponent.K2_SetRelativeLocation` _previewcamera (`SplineComponent.GetLocationAtTime` (`self.CameraSpline`) (`self.PreviewTime`) "Local" true) false false)
      (`SceneComponent.K2_SetWorldRotation` _previewcamera (`KismetMathLibrary.FindLookAtRotation` (`SceneComponent.K2_GetComponentLocation` (`self.PreviewCamera`)) (+ (`self.K2_GetActorLocation`) (`self.CameraFocusPoint`))) false false))))