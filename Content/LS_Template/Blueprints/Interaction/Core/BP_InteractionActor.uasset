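; Base interactable actor for child Blueprints, which override its Interaction event.
; Sphere, box or capsule overlaps register and unregister the actor with BP_LS_GameController when the overlapping actor's instigator is that player controller, and fire begin/end calls.
; HandleInteractionShape sizes the selected shape and destroys the other two.
; Helpers set the prompt widget's text and optional money/energy costs, and toggle its visibility and useable state; interacting hides the prompt.
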(event `self.ReceiveBeginPlay`
  (bind _asbp_ls_game_controller (cast `/Game/LS_Template/Blueprints/Systems/Core/Game/BP_LS_GameController` (`GameplayStatics.GetPlayerController` 0)))
  (set `self.PlayerController` _asbp_ls_game_controller))

(event `/Game/LS_Template/Blueprints/Interaction/Core/BPI_Interaction.Interaction`
  (params (LS_Controller :type "/Game/LS_Template/Blueprints/Systems/Core/Game/BP_LS_GameController Object Reference"))
  ;[1 1 1] Event on interaction. Overriden in child blueprint
  (`self.HidePrompt` false)
  (`self.OnInteraction`))

(event `self.InteractionSphere.OnComponentBeginOverlap`
  (params (OverlappedComponent :type "PrimitiveComponent Object Reference") (OtherActor :type "Actor Object Reference") (OtherComp :type "PrimitiveComponent Object Reference") (OtherBodyIndex :type Integer) (bFromSweep :type Boolean) (SweepResult :type "HitResult Structure (by ref)"))
  ;[1 1 1] Overlap Events
  (bind _asbp_ls_game_controller (`self.IsLST_Controlled?` OtherActor)
    (:`true`
      (message `/Game/LS_Template/Blueprints/Interaction/Core/BPI_Interaction.RegisterInteractable` _asbp_ls_game_controller self)
      (`self.OnBeginOverlap`))))

(event `self.InteractionSphere.OnComponentEndOverlap`
  (params (OverlappedComponent :type "PrimitiveComponent Object Reference") (OtherActor :type "Actor Object Reference") (OtherComp :type "PrimitiveComponent Object Reference") (OtherBodyIndex :type Integer))
  ;[1 1 1] Overlap Events
  (bind _asbp_ls_game_controller (`self.IsLST_Controlled?` OtherActor)
    (:`true`
      (message `/Game/LS_Template/Blueprints/Interaction/Core/BPI_Interaction.UnregisterInteractable` _asbp_ls_game_controller self)
      (`self.OnEndOverlap`))))

(event `self.InteractionBox.OnComponentBeginOverlap`
  (params (OverlappedComponent :type "PrimitiveComponent Object Reference") (OtherActor :type "Actor Object Reference") (OtherComp :type "PrimitiveComponent Object Reference") (OtherBodyIndex :type Integer) (bFromSweep :type Boolean) (SweepResult :type "HitResult Structure (by ref)"))
  ;[1 1 1] Overlap Events
  (bind _asbp_ls_game_controller (`self.IsLST_Controlled?` OtherActor)
    (:`true`
      (message `/Game/LS_Template/Blueprints/Interaction/Core/BPI_Interaction.RegisterInteractable` _asbp_ls_game_controller self)
      (`self.OnBeginOverlap`))))

(event `self.InteractionBox.OnComponentEndOverlap`
  (params (OverlappedComponent :type "PrimitiveComponent Object Reference") (OtherActor :type "Actor Object Reference") (OtherComp :type "PrimitiveComponent Object Reference") (OtherBodyIndex :type Integer))
  ;[1 1 1] Overlap Events
  (bind _asbp_ls_game_controller (`self.IsLST_Controlled?` OtherActor)
    (:`true`
      (message `/Game/LS_Template/Blueprints/Interaction/Core/BPI_Interaction.UnregisterInteractable` _asbp_ls_game_controller self)
      (`self.OnEndOverlap`))))

(event `self.InteractionCapsule.OnComponentBeginOverlap`
  (params (OverlappedComponent :type "PrimitiveComponent Object Reference") (OtherActor :type "Actor Object Reference") (OtherComp :type "PrimitiveComponent Object Reference") (OtherBodyIndex :type Integer) (bFromSweep :type Boolean) (SweepResult :type "HitResult Structure (by ref)"))
  ;[1 1 1] Overlap Events
  (bind _asbp_ls_game_controller (`self.IsLST_Controlled?` OtherActor)
    (:`true`
      (message `/Game/LS_Template/Blueprints/Interaction/Core/BPI_Interaction.RegisterInteractable` _asbp_ls_game_controller self)
      (`self.OnBeginOverlap`))))

(event `self.InteractionCapsule.OnComponentEndOverlap`
  (params (OverlappedComponent :type "PrimitiveComponent Object Reference") (OtherActor :type "Actor Object Reference") (OtherComp :type "PrimitiveComponent Object Reference") (OtherBodyIndex :type Integer))
  ;[1 1 1] Overlap Events
  (bind _asbp_ls_game_controller (`self.IsLST_Controlled?` OtherActor)
    (:`true`
      (message `/Game/LS_Template/Blueprints/Interaction/Core/BPI_Interaction.UnregisterInteractable` _asbp_ls_game_controller self)
      (`self.OnEndOverlap`))))

(fn `HandleInteractionShape`
  (params (SelectedShape :type "/Game/LS_Template/Blueprints/Systems/Enumerations/Interaction/E_InteractionShapes Enum" :default "NewEnumerator0") (SphereRadius :type "Float (double-precision)" :default 100.0) (BoxExtent :type "Vector Structure" :default (10.0 10.0 10.0)) (CapsuleHalfHeight :type "Float (double-precision)" :default 96.0) (CapsuleRadius :type "Float (double-precision)" :default 42.0))
  (bind _interactioncapsule (`self.InteractionCapsule`))
  (set `self.SphereRadius` SphereRadius)
  (set `self.BoxExtent` BoxExtent)
  (set `self.CapsuleHalfHeight` CapsuleHalfHeight)
  (set `self.CapsuleRadius` CapsuleRadius)
  (switch `/Game/LS_Template/Blueprints/Systems/Enumerations/Interaction/E_InteractionShapes` SelectedShape
    (:`NewEnumerator0`
      (`ActorComponent.K2_DestroyComponent` (`self.InteractionBox`))
      (`ActorComponent.K2_DestroyComponent` (`self.InteractionCapsule`))
      (`SphereComponent.SetSphereRadius` (`self.InteractionSphere`) (`self.SphereRadius`) true))
    (:`NewEnumerator1`
      (`ActorComponent.K2_DestroyComponent` (`self.InteractionCapsule`))
      (`ActorComponent.K2_DestroyComponent` (`self.InteractionSphere`))
      (`BoxComponent.SetBoxExtent` (`self.InteractionBox`) (`self.BoxExtent`) true))
    (:`NewEnumerator2`
      (`ActorComponent.K2_DestroyComponent` (`self.InteractionSphere`))
      (`ActorComponent.K2_DestroyComponent` (`self.InteractionBox`))
      (`CapsuleComponent.SetCapsuleHalfHeight` _interactioncapsule (`self.CapsuleHalfHeight`) true)
      (`CapsuleComponent.SetCapsuleRadius` _interactioncapsule (`self.CapsuleRadius`) true))))

(fn `HidePrompt`
  (params (`Visible?` :type Boolean))
  (`SceneComponent.SetVisibility` (`self.Widget`) `Visible?` false)
  (return))

(fn `SetUseable`
  (params (`Useable?` :type Boolean))
  (`SceneComponent.SetHiddenInGame` (`self.Widget`) (not `Useable?`) false)
  (if `Useable?`
    (`self.OnSetUseable`)
    (return)
    (else
      (`self.OnSetUnuseable`)
      (return))))

(fn `SetWidget`
  (params (InteractionText :type Text) (`DisplayCosts?` :type Boolean) (MoneyCost :type Integer) (EnergyCost :type Integer))
  (bind _asw_interaction_prompt (cast `/Game/LS_Template/Blueprints/UI/Interaction/W_InteractionPrompt` (`WidgetComponent.GetUserWidgetObject` (`self.Widget`))))
  (bind _output_get (set `/Game/LS_Template/Blueprints/UI/Interaction/W_InteractionPrompt.InteractionText` InteractionText _asw_interaction_prompt))
  (`TextBlock.SetText` (`/Game/LS_Template/Blueprints/UI/Interaction/W_InteractionPrompt.InteractionPromptText` _asw_interaction_prompt) _output_get)
  (if `DisplayCosts?`
    (set `/Game/LS_Template/Blueprints/UI/Interaction/W_InteractionPrompt.MoneyCost` MoneyCost _asw_interaction_prompt)
    (set `/Game/LS_Template/Blueprints/UI/Interaction/W_InteractionPrompt.EnergyCost` EnergyCost _asw_interaction_prompt)
    (return)
    (else
      (`Widget.SetVisibility` (`/Game/LS_Template/Blueprints/UI/Interaction/W_InteractionPrompt.ActivityEnergyCostText` _asw_interaction_prompt) "Hidden")
      (`Widget.SetVisibility` (`/Game/LS_Template/Blueprints/UI/Interaction/W_InteractionPrompt.ActivityMoneyCostText` _asw_interaction_prompt) "Hidden")
      (return))))

(fn `UserConstructionScript`)