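; Interaction component that tracks registered interactable actors and selects the one the player camera is looking at most directly.
; Each tick it compares the camera forward vector to each actor's direction by dot product, keeping the best above a threshold and toggling its useable state.
; InteractionEvent forwards the controller to the selected actor's Interaction call.
; Initialize stores the camera and adds a dynamic outline post-process material to it.
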(event `self.ReceiveTick`
  (params (DeltaSeconds :type "Float (single-precision)"))
  (`self.UpdateBestInteractionActor`))

(event `InteractionEvent`
  (params (LS_Controller :type "/Game/LS_Template/Blueprints/Systems/Core/Game/BP_LS_GameController Object Reference"))
  (bind _selectedinteractionactor (`self.SelectedInteractionActor`))
  (`/Engine/EditorBlueprintResources/StandardMacros.IsValid` _selectedinteractionactor
    (:`Is Valid`
      (`/Game/LS_Template/Blueprints/Interaction/Core/BP_InteractionActor.Interaction` _selectedinteractionactor LS_Controller))))

(fn `GetBestInteractionActor`
  (locals (LocalInteractionStruct :type "/Game/LS_Template/Blueprints/Systems/Structures/Interaction/S_InteractionActor Structure"))
  (bind _playercamera (`self.PlayerCamera`))
  (bind _localinteractionstruct_dot (break `/Game/LS_Template/Blueprints/Systems/Structures/Interaction/S_InteractionActor` (`local.LocalInteractionStruct`)))
  (bind (_localinteractionstruct_dot_2 _localinteractionstruct_interactionactor) (break `/Game/LS_Template/Blueprints/Systems/Structures/Interaction/S_InteractionActor` (`local.LocalInteractionStruct`)))
  (set `local.LocalInteractionStruct` (make `/Game/LS_Template/Blueprints/Systems/Structures/Interaction/S_InteractionActor` -1.0))
  (for _array_element (`self.Interactables`)
    (bind _returnvalue (`KismetMathLibrary.Dot_VectorVector` (`KismetMathLibrary.Normal` (- (`Actor.K2_GetActorLocation` _array_element) (`SceneComponent.K2_GetComponentLocation` _playercamera))) (`SceneComponent.GetForwardVector` _playercamera)))
    (if (and (> _returnvalue 0.8) (> _returnvalue _localinteractionstruct_dot))
      (set `local.LocalInteractionStruct` (make `/Game/LS_Template/Blueprints/Systems/Structures/Interaction/S_InteractionActor` _returnvalue _array_element))))
  (`/Engine/EditorBlueprintResources/StandardMacros.IsValid` _localinteractionstruct_interactionactor
    (:`Is Valid`
      (`self.SetBestInteractionActor` _localinteractionstruct_interactionactor))
    (:`Is Not Valid`
      (`self.SetBestInteractionActor` null)))
  (return))

(fn `HandleRegisterInteractionActor`
  (params (InteractionActor :type "/Game/LS_Template/Blueprints/Interaction/Core/BP_InteractionActor Object Reference (by ref)"))
  (`KismetArrayLibrary.Array_AddUnique` (`self.Interactables`) InteractionActor)
  (return))

(fn `HandleUnregisterInteractionActor`
  (params (InteractionActor :type "/Game/LS_Template/Blueprints/Interaction/Core/BP_InteractionActor Object Reference"))
  (`KismetArrayLibrary.Array_RemoveItem` (`self.Interactables`) InteractionActor)
  (return))

(fn `Initialize`
  (params (PlayerCamera :type "CameraComponent Object Reference"))
  (bind _output_get (set `self.PlayerCamera` PlayerCamera))
  (bind _returnvalue (`KismetMaterialLibrary.CreateDynamicMaterialInstance` "/Game/LS_Template/Blueprints/Interaction/Core/M_PP_Outline.M_PP_Outline"))
  (bind _output_get_2 (set `self.OutlineDynamat` _returnvalue))
  (`CameraComponent.AddOrUpdateBlendable` _output_get _output_get_2 1.0)
  (return))

(fn `SetBestInteractionActor`
  (params (InteractionActor :type "/Game/LS_Template/Blueprints/Interaction/Core/BP_InteractionActor Object Reference"))
  (`/Engine/EditorBlueprintResources/StandardMacros.IsValid` InteractionActor
    (:`Is Valid`
      (if (!= InteractionActor (`self.SelectedInteractionActor`))
        (bind _selectedinteractionactor (`self.SelectedInteractionActor`)
          (:`then`
            (`/Game/LS_Template/Blueprints/Interaction/Core/BP_InteractionActor.SetUseable` _selectedinteractionactor false))
          (:`else`
            _)))
      (bind _output_get (set `self.SelectedInteractionActor` InteractionActor))
      (`/Game/LS_Template/Blueprints/Interaction/Core/BP_InteractionActor.SetUseable` _output_get true)
      (return))
    (:`Is Not Valid`
      (bind _selectedinteractionactor_2 (`self.SelectedInteractionActor`)
        (:`then`
          (`/Game/LS_Template/Blueprints/Interaction/Core/BP_InteractionActor.SetUseable` _selectedinteractionactor_2 false)
          (set `self.SelectedInteractionActor` null)
          (return))
        (:`else`)))))

(fn `UpdateBestInteractionActor`
  (if (> (`KismetArrayLibrary.Array_Length` (`self.Interactables`)) 0)
    (`self.GetBestInteractionActor`)
    (return)
    (else
      (`self.SetBestInteractionActor` null)
      (return))))