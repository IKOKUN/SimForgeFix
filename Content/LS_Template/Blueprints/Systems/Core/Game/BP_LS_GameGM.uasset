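; Game mode that picks where the player spawns, using level switcher actors in the loaded level.
; ChoosePlayerStart finds the BP_LevelSwitcher whose SpawnPointName matches the one stored in the LS game instance and returns its child actor as the start.
; If no switcher matches or none exist, it falls back to the first PlayerStart found.
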(fn `ChoosePlayerStart`
  (params (Player :type "Controller Object Reference"))
  (returns (ReturnValue :type "Actor Object Reference"))
  (locals (`LocalFound?` :type Boolean) (LocalSelectedSpawnPoint :type "Actor Object Reference"))
  (bind _outactors (`GameplayStatics.GetAllActorsOfClass` "/Game/LS_Template/Blueprints/Travels/BP_LevelSwitcher.BP_LevelSwitcher_C"))
  (if (> (`KismetArrayLibrary.Array_Length` _outactors) 0)
    (for _array_element _outactors
      (if (== (`/Game/LS_Template/Blueprints/Travels/BP_LevelSwitcher.SpawnPointName` _array_element) (`/Game/LS_Template/Blueprints/Systems/Core/LS_Instance.SpawnPointName` (`/Game/LS_Template/Blueprints/Systems/Core/BPL_Functions.Get_LST_Instance`)))
        (set `local.LocalFound?` true)
        (set `local.LocalSelectedSpawnPoint` (`ChildActorComponent.ChildActor` (`/Game/LS_Template/Blueprints/Travels/BP_LevelSwitcher.ChildActor` _array_element)))
        (break))))
  (if (`local.LocalFound?`)
    (return (`local.LocalSelectedSpawnPoint`))
    (else
      ;[1 1 1] Failsafe : If a spawn point wasn't found, spawn on a player start
      (bind _outactors_2 (`GameplayStatics.GetAllActorsOfClass` "/Script/Engine.PlayerStart"))
      (return (`|GetArrayItem` _outactors_2)))))

(fn `UserConstructionScript`)