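; Player controller for the life-sim template that sets up the HUD and interaction component, fades in and saves on BeginPlay.
; It routes input to HUD panels, the pause menu and BPC_Interaction, which is initialized with the third-person character's camera.
; Housing input moves the selected item by enabling its tick while held, rotates it, or returns it to inventory.
; Hardwired debug keys exercise time, saving, stats, money, mood and items.
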(event `Key|T`
  (params (Key :type "Key Structure"))
  ;[0.9948 0 0] DEBUG INPUTS
  (:`Pressed`
    (`/Game/LS_Template/Blueprints/Systems/Core/BPL_Functions.AdvanceDayTime` false "NewEnumerator2")))

(event `Key|A_AccentGrave`
  (params (Key :type "Key Structure"))
  ;[0.9948 0 0] DEBUG INPUTS
  (:`Pressed`
    (`/Game/LS_Template/Blueprints/Systems/Core/BPL_Functions.SaveGame` false)))

(event `Key|R`
  (params (Key :type "Key Structure"))
  ;[0.9948 0 0] DEBUG INPUTS
  (:`Pressed`
    (`/Game/LS_Template/Blueprints/Systems/Core/BPL_Functions.GainStatLevel` "NewEnumerator7")))

(event `Key|Y`
  (params (Key :type "Key Structure"))
  ;[0.9948 0 0] DEBUG INPUTS
  (:`Pressed`
    (`/Game/LS_Template/Blueprints/Systems/Core/BPL_Functions.GainStatExperience` "NewEnumerator4" 64.0)))

(event `Key|F`
  (params (Key :type "Key Structure"))
  ;[0.9948 0 0] DEBUG INPUTS
)

(event `self.ReceiveBeginPlay`
  (`|ExecutionSequence`
    (:`then_0`
      (`/Game/LS_Template/Blueprints/Systems/Core/LS_Instance.SetInventoryMaxSlots` (`/Game/LS_Template/Blueprints/Systems/Core/BPL_Functions.Get_LST_Instance`)))
    (:`then_1`
      (bind _returnvalue (`|CreateWidget` "/Game/LS_Template/Blueprints/UI/W_PlayerHUD.W_PlayerHUD_C"))
      (bind _output_get (set `self.W_PlayerHUD` _returnvalue))
      (`UserWidget.AddToViewport` _output_get 0)
      (`WidgetBlueprintLibrary.SetInputMode_GameOnly` self))
    (:`then_2`
      ;[0.9948 0 0] Cast to your own character here and plug its own camera in the "Initialize node"
      (bind _asthird_person_character (cast `/Game/LS_Template/EpicContent/CharacterExampleContent/ThirdPersonCharacter` (`GameplayStatics.GetPlayerCharacter` 0)))
      (`/Game/LS_Template/Blueprints/Interaction/Core/BPC_Interaction.Initialize` (`self.BPC_Interaction`) (`/Game/LS_Template/EpicContent/CharacterExampleContent/ThirdPersonCharacter.FollowCamera` _asthird_person_character)))
    (:`then_3`
      (`/Game/LS_Template/Blueprints/Systems/Core/BPL_Functions.CameraFadeIn` 2.0)
      (`/Game/LS_Template/Blueprints/Systems/Core/BPL_Functions.SaveGame` false))))

(event `Key|I`
  (params (Key :type "Key Structure"))
  ;[0.9948 0 0] DEBUG INPUTS
  (:`Pressed`
    (`/Game/LS_Template/Blueprints/Systems/Core/BPL_Functions.AddMoney` 100)))

(event `Key|RightParantheses`
  (params (Key :type "Key Structure"))
  ;[0.9948 0 0] DEBUG INPUTS
  (:`Pressed`
    (`/Engine/EditorBlueprintResources/StandardMacros.FlipFlop`
      (:`A`
        (`/Game/LS_Template/Blueprints/Systems/Core/BPL_Functions.RemoveMood` 11.0))
      (:`B`
        (`/Game/LS_Template/Blueprints/Systems/Core/BPL_Functions.AddMood` 5.0)))))

(event `Key|O`
  (params (Key :type "Key Structure"))
  ;[0.9948 0 0] DEBUG INPUTS
  (:`Pressed`
    (`/Game/LS_Template/Blueprints/Systems/Core/BPL_Functions.AddItemToInventory` "Present" 50)))

(event `InputAction|SelectHousingItem`
  (params (Key :type "Key Structure"))
  (bind _selectedhouseitem (`self.SelectedHouseItem`))
  (bind _sm_housingmesh (`/Game/LS_Template/Blueprints/Housing/BP_Housing.SM_HousingMesh` _selectedhouseitem))
  ;[1 1 1] Housing Inputs
  ;;[1 1 1] Select Housing Item
  (:`Pressed`
    (`/Engine/EditorBlueprintResources/StandardMacros.IsValid` _selectedhouseitem
      (:`Is Valid`
        (`self.SetActorTickEnabled` _selectedhouseitem true)
        (`/Game/LS_Template/Blueprints/Housing/BP_Housing.DisablePawnCollisionChannel` _selectedhouseitem true)
        (`PrimitiveComponent.SetRenderCustomDepth` _sm_housingmesh true))))
  (:`Released`
    (`/Engine/EditorBlueprintResources/StandardMacros.IsValid` _selectedhouseitem
      (:`Is Valid`
        (`self.SetActorTickEnabled` _selectedhouseitem false)
        (`/Game/LS_Template/Blueprints/Housing/BP_Housing.DisablePawnCollisionChannel` _selectedhouseitem false)
        (`PrimitiveComponent.SetRenderCustomDepth` _sm_housingmesh false)
        (set `self.SelectedHouseItem` null)))))

(event `InputAction|DisplayInventoryHUD`
  (params (Key :type "Key Structure"))
  ;[1 1 1] Displays Inventory HUD
  (:`Pressed`
    (if (not (`self.IsInteractingWithNPC?`))
      (`/Game/LS_Template/Blueprints/UI/W_PlayerHUD.DisplayHUD` (`self.W_PlayerHUD`) false true))))

(event `/Game/LS_Template/Blueprints/Interaction/Core/BPI_Interaction.RegisterInteractable`
  (params (Interactable :type "/Game/LS_Template/Blueprints/Interaction/Core/BP_InteractionActor Object Reference"))
  ;[1 1 1] Interaction Events
  (`/Game/LS_Template/Blueprints/Interaction/Core/BPC_Interaction.HandleRegisterInteractionActor` (`self.BPC_Interaction`) Interactable))

(event `InputAction|RemoveHousingItem`
  (params (Key :type "Key Structure"))
  (bind _selectedhouseitem (`self.SelectedHouseItem`))
  (bind _interactionactor (`/Game/LS_Template/Blueprints/Housing/BP_Housing.InteractionActor` _selectedhouseitem))
  (bind _iteminfo_itemrowname (break `/Game/LS_Template/Blueprints/Systems/Structures/Items/S_ItemInfo` (`/Game/LS_Template/Blueprints/Housing/BP_Housing.ItemInfo` _selectedhouseitem)))
  ;[1 1 1] Housing Inputs
  ;;[1 1 1] Remove Housing Item
  (:`Pressed`
    (`/Engine/EditorBlueprintResources/StandardMacros.IsValid` _selectedhouseitem
      (:`Is Valid`
        (if (`self.IsActorTickEnabled` _selectedhouseitem)
          (`/Game/LS_Template/Blueprints/Systems/Core/BPL_Functions.AddItemToInventory` _iteminfo_itemrowname 1)
          (`/Engine/EditorBlueprintResources/StandardMacros.IsValid` _interactionactor
            (:`Is Valid`
              (`self.K2_DestroyActor` _interactionactor))
            (:`Is Not Valid`
              _))
          (`self.K2_DestroyActor` _selectedhouseitem))))))

(event `/Game/LS_Template/Blueprints/Interaction/Core/BPI_Interaction.UnregisterInteractable`
  (params (Interactable :type "/Game/LS_Template/Blueprints/Interaction/Core/BP_InteractionActor Object Reference"))
  ;[1 1 1] Interaction Events
  (`/Game/LS_Template/Blueprints/Interaction/Core/BPC_Interaction.HandleUnregisterInteractionActor` (`self.BPC_Interaction`) Interactable))

(event `InputAction|DisplayStatsHUD`
  (params (Key :type "Key Structure"))
  ;[1 1 1] Displays Stats HUD
  (:`Pressed`
    (if (not (`self.IsInteractingWithNPC?`))
      (`/Game/LS_Template/Blueprints/UI/W_PlayerHUD.DisplayHUD` (`self.W_PlayerHUD`) false false))))

(event `InputAction|Interaction`
  (params (Key :type "Key Structure"))
  ;[1 1 1] Interaction Events
  (:`Pressed`
    (if (not (`self.IsInteractingWithNPC?`))
      (`/Game/LS_Template/Blueprints/Interaction/Core/BPC_Interaction.InteractionEvent` (`self.BPC_Interaction`) self))))

(event `InputAxis|RotateHousingItem`
  (params (AxisValue :type "Float (single-precision)"))
  (bind _selectedhouseitem (`self.SelectedHouseItem`))
  (bind (_iteminfo_itemrowname _iteminfo_itemname _iteminfo_itemdescription _iteminfo_itemtype _iteminfo_clothestype _iteminfo_itemrarity _iteminfo_itemicon _iteminfo_itemsound _iteminfo_simulatephysics_ _iteminfo_itemmesh _iteminfo_itemskeletalmesh _iteminfo_itemprice _iteminfo_itemamount _iteminfo_gaindetails _iteminfo_housingdetails) (break `/Game/LS_Template/Blueprints/Systems/Structures/Items/S_ItemInfo` (`/Game/LS_Template/Blueprints/Housing/BP_Housing.ItemInfo` _selectedhouseitem)))
  ;[1 1 1] Housing Inputs
  ;;[1 1 1] Rotate housing mesh (only if it isn't a wall item)
  (`/Engine/EditorBlueprintResources/StandardMacros.IsValid` _selectedhouseitem
    (:`Is Valid`
      (if (`.WallItem?_6_C5E5A9D743B25C281B3AA4AC2D4D0D46` (break `/Game/LS_Template/Blueprints/Systems/Structures/Housing/S_HousingDetails` _iteminfo_housingdetails))
        (`/Game/LS_Template/Blueprints/Housing/BP_Housing.RotateWallMesh` _selectedhouseitem AxisValue)
        (else
          (`/Game/LS_Template/Blueprints/Housing/BP_Housing.RotateMesh` _selectedhouseitem AxisValue))))))

(event `InputAction|PauseMenu`
  (params (Key :type "Key Structure"))
  ;[1 1 1] Display options menu
  (:`Pressed`
    (`self.DisplayPauseMenu`)))

(event `DisplayPauseMenu`
  (bind _w_playerhud (`/Game/LS_Template/Blueprints/Systems/Core/BPL_Functions.Get_LST_PlayerHUD`))
  ;[1 1 1] Display options menu
  (`/Engine/EditorBlueprintResources/StandardMacros.IsValid` (`self.W_PauseMenu`)
    (:`Is Valid`
      _)
    (:`Is Not Valid`
      (bind _returnvalue (`|CreateWidget` "/Game/LS_Template/Blueprints/UI/Settings/W_PauseMenu.W_PauseMenu_C"))
      (set `self.W_PauseMenu` _returnvalue)))
  (`UserWidget.AddToViewport` (`self.W_PauseMenu`) 0)
  (if (`/Game/LS_Template/Blueprints/UI/W_PlayerHUD.IsVisible?` _w_playerhud)
    (`/Game/LS_Template/Blueprints/UI/W_PlayerHUD.DisplayHUD` _w_playerhud true false))
  (set `self.bShowMouseCursor` true)
  (`WidgetBlueprintLibrary.SetInputMode_UIOnlyEx` self (`self.W_PauseMenu`)))

(fn `UserConstructionScript`)