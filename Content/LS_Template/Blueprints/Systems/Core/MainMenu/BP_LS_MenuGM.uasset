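; BP_LS_MenuGM is the main menu game mode, which applies settings and shows the menu screens.
; On BeginPlay it loads and applies settings through the LST game instance.
; Separate events show the main, save and options menus, each creating its widget on first use, caching it and adding it to the viewport.
; The options menu uses the settings widget, created with InGame set to false.
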(event `self.ReceiveBeginPlay`
  (bind _lst_instance (`/Game/LS_Template/Blueprints/Systems/Core/BPL_Functions.Get_LST_Instance`))
  (`/Game/LS_Template/Blueprints/Systems/Core/LS_Instance.LoadSettings` _lst_instance)
  (`/Game/LS_Template/Blueprints/Systems/Core/LS_Instance.ApplySettings` _lst_instance))

(event `ShowMainMenu`
  (`/Engine/EditorBlueprintResources/StandardMacros.IsValid` (`self.W_MainMenu`)
    (:`Is Valid`
      _)
    (:`Is Not Valid`
      (bind _returnvalue (`|CreateWidget` "/Game/LS_Template/Blueprints/UI/MainMenu/W_MainMenu.W_MainMenu_C"))
      (set `self.W_MainMenu` _returnvalue)))
  (`UserWidget.AddToViewport` (`self.W_MainMenu`) 0))

(event `ShowSaveMenu`
  (`/Engine/EditorBlueprintResources/StandardMacros.IsValid` (`self.W_SaveMenu`)
    (:`Is Valid`
      _)
    (:`Is Not Valid`
      (bind _returnvalue (`|CreateWidget` "/Game/LS_Template/Blueprints/UI/MainMenu/W_SaveMenu.W_SaveMenu_C"))
      (set `self.W_SaveMenu` _returnvalue)))
  (`UserWidget.AddToViewport` (`self.W_SaveMenu`) 0))

(event `ShowOptionsMenu`
  (`/Engine/EditorBlueprintResources/StandardMacros.IsValid` (`self.W_SettingsMenu`)
    (:`Is Valid`
      _)
    (:`Is Not Valid`
      (bind _returnvalue (`|CreateWidget` "/Game/LS_Template/Blueprints/UI/Settings/W_SettingsMenu.W_SettingsMenu_C" null false))
      (set `self.W_SettingsMenu` _returnvalue)))
  (`UserWidget.AddToViewport` (`self.W_SettingsMenu`) 0))

(fn `UserConstructionScript`)