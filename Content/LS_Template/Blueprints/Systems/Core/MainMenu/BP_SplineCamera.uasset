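; BP_SplineCamera is a main menu camera actor that flies its camera along an editable spline.
; On BeginPlay a timeline drives an alpha, scaled by spline length, to set the camera's world location and rotation from the spline each update.
; The construction script applies the closed-loop option and sets the timeline rate to the inverse of PlayRate, so larger values slow the move.
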(event `self.ReceiveBeginPlay`
  (bind _spline (`self.Spline`))
  (bind (_direction _cameraalpha) (`Timeline|CameraTL` :!via `PlayFromStart`)
    (:`Update`
      (bind _returnvalue (* (`SplineComponent.GetSplineLength` _spline) _cameraalpha))
      (`SceneComponent.K2_SetWorldTransform` (`self.CameraComponent`) (`KismetMathLibrary.MakeTransform` (`SplineComponent.GetLocationAtDistanceAlongSpline` _spline _returnvalue "World") (`SplineComponent.GetRotationAtDistanceAlongSpline` _spline _returnvalue "World")) false false))))

(fn `UserConstructionScript`
  (`SplineComponent.SetClosedLoop` (`self.Spline`) (`self.ClosedLoop?`) true)
  (`TimelineComponent.SetPlayRate` (`self.CameraTL`) (/ 1.0 (`self.PlayRate`))))