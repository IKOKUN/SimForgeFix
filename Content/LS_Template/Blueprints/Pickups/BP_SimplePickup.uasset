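; BP_SimplePickup is a world pickup that grants a configurable item and amount to the inventory when the player walks into it.
; The construction script looks up the item row in the item datatable to set the displayed mesh and material, and applies the sphere radius.
; Overlap by a ThirdPersonCharacter passes through a DoOnce, adds the item, then destroys the pickup.
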(event `self.SphereCollision.OnComponentBeginOverlap`
  (params (OverlappedComponent :type "PrimitiveComponent Object Reference") (OtherActor :type "Actor Object Reference") (OtherComp :type "PrimitiveComponent Object Reference") (OtherBodyIndex :type Integer) (bFromSweep :type Boolean) (SweepResult :type "HitResult Structure (by ref)"))
  ;[1 0 0] Cast to your own character
  ; if you don't use the standard one
  (cast `/Game/LS_Template/EpicContent/CharacterExampleContent/ThirdPersonCharacter` OtherActor)
  (`/Engine/EditorBlueprintResources/StandardMacros.DoOnce` false
    (:`Completed`
      (`/Game/LS_Template/Blueprints/Systems/Core/BPL_Functions.AddItemToInventory` (`self.ItemToGrant`) (`self.ItemAmount`))
      (`self.K2_DestroyActor`))))

(fn `UserConstructionScript`
  (bind _sm_pickup (`self.SM_PickUp`))
  (bind (_itemrowname _itemname _itemdescription _itemtype _clothestype _itemrarity _itemicon _itemsound _simulatephysics_ _itemmesh) (break `/Game/LS_Template/Blueprints/Systems/Structures/Items/S_ItemInfo` (`/Game/LS_Template/Blueprints/Systems/Core/BPL_Functions.GetItemInfoInDatatable` (`self.ItemToGrant`))))
  (`StaticMeshComponent.SetStaticMesh` _sm_pickup _itemmesh)
  (`PrimitiveComponent.SetMaterial` _sm_pickup 0 (`StaticMesh.GetMaterial` _itemmesh 0))
  (`SphereComponent.SetSphereRadius` (`self.SphereCollision`) (`self.SphereRadius`) true))