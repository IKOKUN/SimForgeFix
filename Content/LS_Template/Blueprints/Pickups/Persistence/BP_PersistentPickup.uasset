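; Persistent item pickup that grants an inventory item when the player character overlaps its sphere, then destroys itself.
; The construction script takes the mesh and material from the item data table row and applies the sphere radius.
; On pickup it records its PickUpID in the game instance's PersistenceData map, keyed by level name.
; Shortly after BeginPlay it checks that map and destroys itself if already collected, supporting loaded games.
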(event `self.ReceiveBeginPlay`
  ;[1 0 0] Needed for load game purposes
  (`KismetSystemLibrary.Delay` 0.2)
  (bind _alreadypickedup_ (`self.HasAlreadyBeenPickedUp?`))
  (if _alreadypickedup_
    (`self.K2_DestroyActor`)))

(event `self.SphereCollision.OnComponentBeginOverlap`
  (params (OverlappedComponent :type "PrimitiveComponent Object Reference") (OtherActor :type "Actor Object Reference") (OtherComp :type "PrimitiveComponent Object Reference") (OtherBodyIndex :type Integer) (bFromSweep :type Boolean) (SweepResult :type "HitResult Structure (by ref)"))
  ;[1 0 0] Cast to your own character
  ; if you don't use the standard one
  (cast `/Game/LS_Template/EpicContent/CharacterExampleContent/ThirdPersonCharacter` OtherActor)
  (`/Engine/EditorBlueprintResources/StandardMacros.DoOnce` false
    (:`Completed`
      (`self.OnPickedUp`)
      (`/Game/LS_Template/Blueprints/Systems/Core/BPL_Functions.AddItemToInventory` (`self.ItemToGrant`) (`self.ItemAmount`))
      (`self.K2_DestroyActor`))))

(fn `HasAlreadyBeenPickedUp?`
  (returns (`AlreadyPickedUp?` :type Boolean))
  (locals (LocalPersistenceData :type "Map of Name to /Game/LS_Template/Blueprints/Pickups/Persistence/S_PickupInfos Structure"))
  (set `local.LocalPersistenceData` (`/Game/LS_Template/Blueprints/Systems/Core/LS_Instance.PersistenceData` (`/Game/LS_Template/Blueprints/Systems/Core/BPL_Functions.Get_LST_Instance`)))
  (bind _returnvalue (`GameplayStatics.GetCurrentLevelName` true))
  (bind (_value _returnvalue_2) (`BlueprintMapLibrary.Map_Find` (`local.LocalPersistenceData`) (`KismetStringLibrary.Conv_StringToName` _returnvalue)))
  (if _returnvalue_2
    (return (`BlueprintSetLibrary.Set_Contains` (`.PickUp_ID_3_FEC83DDA4D7F7CA6329F35BC542F03C7` (break `/Game/LS_Template/Blueprints/Pickups/Persistence/S_PickupInfos` _value)) (`self.PickUpID`)))
    (else
      (return false))))

(fn `OnPickedUp`
  (locals (LocalPersistenceData :type "Map of Name to /Game/LS_Template/Blueprints/Pickups/Persistence/S_PickupInfos Structure") (LocalLevelName :type Name :default "None") (LocalPickUpIDs :type "Set of Integer"))
  (bind (_value _returnvalue) (`BlueprintMapLibrary.Map_Find` (`local.LocalPersistenceData`) (`local.LocalLevelName`)))
  (set `local.LocalPersistenceData` (`/Game/LS_Template/Blueprints/Systems/Core/LS_Instance.PersistenceData` (`/Game/LS_Template/Blueprints/Systems/Core/BPL_Functions.Get_LST_Instance`)))
  (bind _returnvalue_2 (`GameplayStatics.GetCurrentLevelName` true))
  (set `local.LocalLevelName` (`KismetStringLibrary.Conv_StringToName` _returnvalue_2))
  (if _returnvalue
    (bind _output_get (set `local.LocalPickUpIDs` (`.PickUp_ID_3_FEC83DDA4D7F7CA6329F35BC542F03C7` (break `/Game/LS_Template/Blueprints/Pickups/Persistence/S_PickupInfos` _value))))
    (`BlueprintSetLibrary.Set_Add` _output_get (`self.PickUpID`))
    (bind _structout (setmembers `/Game/LS_Template/Blueprints/Pickups/Persistence/S_PickupInfos` :`StructRef` _value :`PickUp_ID` (`local.LocalPickUpIDs`) :`ItemToGrant` (`self.ItemToGrant`) :`ItemAmount` (`self.ItemAmount`)))
    (`BlueprintMapLibrary.Map_Add` (`/Game/LS_Template/Blueprints/Systems/Core/LS_Instance.PersistenceData` (`/Game/LS_Template/Blueprints/Systems/Core/BPL_Functions.Get_LST_Instance`)) (`local.LocalLevelName`) _structout)
    (return)
    (else
      (`BlueprintMapLibrary.Map_Add` (`/Game/LS_Template/Blueprints/Systems/Core/LS_Instance.PersistenceData` (`/Game/LS_Template/Blueprints/Systems/Core/BPL_Functions.Get_LST_Instance`)) (`local.LocalLevelName`) (make `/Game/LS_Template/Blueprints/Pickups/Persistence/S_PickupInfos` (`|MakeSet` (`self.PickUpID`)) (`self.ItemToGrant`) (`self.ItemAmount`)))
      (return))))

(fn `UserConstructionScript`
  (bind _sm_pickup (`self.SM_PickUp`))
  (bind (_itemrowname _itemname _itemdescription _itemtype _clothestype _itemrarity _itemicon _itemsound _simulatephysics_ _itemmesh) (break `/Game/LS_Template/Blueprints/Systems/Structures/Items/S_ItemInfo` (`/Game/LS_Template/Blueprints/Systems/Core/BPL_Functions.GetItemInfoInDatatable` (`self.ItemToGrant`))))
  (`StaticMeshComponent.SetStaticMesh` _sm_pickup _itemmesh)
  (`PrimitiveComponent.SetMaterial` _sm_pickup 0 (`StaticMesh.GetMaterial` _itemmesh 0))
  (`SphereComponent.SetSphereRadius` (`self.SphereCollision`) (`self.SphereRadius`) true))