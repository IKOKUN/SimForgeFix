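; Level travel trigger that moves the player to another map, or to the game instance's housing map when flagged.
; On player overlap it toggles off open inventory or stats UI, stores the destination spawn point name, saves, fades the camera, then opens the level.
; The construction script sizes the box, writes a descriptive label, and positions and names a child BP_SpawnPoint.
; The housing spawn point override is unconnected.
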(event `self.ReceiveBeginPlay`)

(event `self.Box.OnComponentBeginOverlap`
  (params (OverlappedComponent :type "PrimitiveComponent Object Reference") (OtherActor :type "Actor Object Reference") (OtherComp :type "PrimitiveComponent Object Reference") (OtherBodyIndex :type Integer) (bFromSweep :type Boolean) (SweepResult :type "HitResult Structure (by ref)"))
  (bind _w_playerhud (`/Game/LS_Template/Blueprints/Systems/Core/BPL_Functions.Get_LST_PlayerHUD`))
  (if (== OtherActor (`GameplayStatics.GetPlayerCharacter` 0))
    (if (`/Game/LS_Template/Blueprints/UI/W_PlayerHUD.IsInventoryVisible` _w_playerhud)
      (`/Game/LS_Template/Blueprints/UI/W_PlayerHUD.DisplayHUD` _w_playerhud false true))
    (if (`/Game/LS_Template/Blueprints/UI/W_PlayerHUD.IsStatsVisible` _w_playerhud)
      (`/Game/LS_Template/Blueprints/UI/W_PlayerHUD.DisplayHUD` _w_playerhud false false)
      (`/Game/LS_Template/Blueprints/UI/W_PlayerHUD.DisplayHUD` _w_playerhud false false))
    (set `/Game/LS_Template/Blueprints/Systems/Core/LS_Instance.SpawnPointName` (`self.DestinationSpawnPoint`) (`/Game/LS_Template/Blueprints/Systems/Core/BPL_Functions.Get_LST_Instance`))
    (`/Game/LS_Template/Blueprints/Systems/Core/BPL_Functions.SaveGame` false)
    (`/Game/LS_Template/Blueprints/Systems/Core/BPL_Functions.CameraFadeOut` 1.0)
    (`KismetSystemLibrary.Delay` 1.0)
    (`GameplayStatics.OpenLevel` (select `bool` (`self.UsedForHousing?`) :`false` (`self.LevelToOpen`) :`true` (`KismetStringLibrary.Conv_StringToName` (`/Game/LS_Template/Blueprints/Systems/Core/LS_Instance.HousingMapName` (`/Game/LS_Template/Blueprints/Systems/Core/BPL_Functions.Get_LST_Instance`)))))))

(fn `UserConstructionScript`
  (bind _childactor (`self.ChildActor`))
  (`TextRenderComponent.K2_SetText` (`self.TextRender`) (`|FormatText` "Spawn Point Name : {SpawnName} \n \nIt will open {MapName} and spawns \nthe player at {SpawnPoint}" (`KismetTextLibrary.Conv_NameToText` (`self.SpawnPointName`)) (select `bool` (`self.UsedForHousing?`) :`false` (`KismetTextLibrary.Conv_NameToText` (`self.LevelToOpen`)) :`true` "the housing map in LS_Instance") (select `bool` (`self.UsedForHousing?`) :`false` (`KismetTextLibrary.Conv_NameToText` (`self.DestinationSpawnPoint`)) :`true` "the housing spawn point in LS_Instance")))
  (`BoxComponent.SetBoxExtent` (`self.Box`) (`self.BoxExtent`) true)
  (`SceneComponent.SetHiddenInGame` (`self.Box`) (`self.HideBoxAndText?`) false)
  (`SceneComponent.SetHiddenInGame` (`self.TextRender`) (`self.HideBoxAndText?`) false)
  (`SceneComponent.K2_SetRelativeLocationAndRotation` _childactor (`self.SpawnPointLocation`) (`self.SpawnPointRotation`) false false)
  (bind _asbp_spawn_point (cast `/Game/LS_Template/Blueprints/Travels/BP_SpawnPoint` (`ChildActorComponent.ChildActor` _childactor)))
  (set `/Game/LS_Template/Blueprints/Travels/BP_SpawnPoint.SpawnPointName` (`self.SpawnPointName`) _asbp_spawn_point))