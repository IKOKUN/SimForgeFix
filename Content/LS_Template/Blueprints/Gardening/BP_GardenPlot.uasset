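; Garden plot actor where the player plants seeds and harvests the grown crop into the inventory.
; Plot state lives in the LST game instance's GardeningPlots map, keyed by PlotIndex and stamped with the planting date.
; A child InteractionActor drives prompt and outline; interacting harvests ripe plants, otherwise opens the gardening menu and disables movement.
; UpdateGardenPlot scales the plant mesh by days left before harvest and refreshes the prompt text.
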(event `self.ReceiveBeginPlay`
  (bind _interactionactor (`self.InteractionActor`))
  (bind (_value _returnvalue) (`BlueprintMapLibrary.Map_Find` (`/Game/LS_Template/Blueprints/Systems/Core/LS_Instance.GardeningPlots` (`/Game/LS_Template/Blueprints/Systems/Core/BPL_Functions.Get_LST_Instance`)) (`self.PlotIndex`)))
  (`KismetSystemLibrary.Delay` 0.2)
  (`self.UpdateGardenPlot`)
  (add `/Game/LS_Template/Blueprints/Interaction/Core/BP_InteractionActor.OnInteraction` _interactionactor (delegate `OnInteractionEvent`))
  (add `/Game/LS_Template/Blueprints/Interaction/Core/BP_InteractionActor.OnSetUseable` _interactionactor (delegate `EventOnUseable`))
  (add `/Game/LS_Template/Blueprints/Interaction/Core/BP_InteractionActor.OnSetUnuseable` _interactionactor (delegate `EventOnUnuseable`))
  (if _returnvalue
    (`StaticMeshComponent.SetStaticMesh` (`self.SM_PlantMesh`) (`.PlantMesh_10_4DE856D64CF4D381BC45BC8CA68FB0C7` (break `/Game/LS_Template/Blueprints/Systems/Structures/Gardening/S_GardenDetails` (`.GardeningDetails_96_050839D542312D15C483939103ED3120` (break `/Game/LS_Template/Blueprints/Systems/Structures/Items/S_ItemInfo` _value)))))))

(event `EventOnUseable`
  (`self.SetOutline?` true))

(event `EventOnUnuseable`
  (`self.SetOutline?` false))

(event `OnInteractionEvent`
  (`self.OnInteraction`))

(event `OnInteraction`
  (bind _w_playerhud (`/Game/LS_Template/Blueprints/Systems/Core/BPL_Functions.Get_LST_PlayerHUD`))
  (bind (_plantmesh _dateplanted _growthdays _daysbeforeharvest _harvesteditemrowname _harvestedamount) (break `/Game/LS_Template/Blueprints/Systems/Structures/Gardening/S_GardenDetails` (`.GardeningDetails_96_050839D542312D15C483939103ED3120` (break `/Game/LS_Template/Blueprints/Systems/Structures/Items/S_ItemInfo` (`BlueprintMapLibrary.Map_Find` (`/Game/LS_Template/Blueprints/Systems/Core/LS_Instance.GardeningPlots` (`/Game/LS_Template/Blueprints/Systems/Core/BPL_Functions.Get_LST_Instance`)) (`self.PlotIndex`))))))
  (if (and (<= _daysbeforeharvest 0) (`KismetSystemLibrary.IsValid` _plantmesh))
    ;[1 1 1] If true, harvest and empties the garden plot
    (`/Game/LS_Template/Blueprints/Systems/Core/BPL_Functions.AddItemToInventory` _harvesteditemrowname _harvestedamount)
    (`self.EmptyGardenPlot`)
    (else
      ;[1 1 1] If false, calls the garden menu
      (if (not (`/Game/LS_Template/Blueprints/UI/W_PlayerHUD.IsVisible?` _w_playerhud))
        (`/Game/LS_Template/Blueprints/UI/W_PlayerHUD.DisplayHUD` _w_playerhud false))
      (`/Game/LS_Template/Blueprints/Systems/Core/LS_Instance.ShowGardeningMenu` (`/Game/LS_Template/Blueprints/Systems/Core/BPL_Functions.Get_LST_Instance`) self)
      (`CharacterMovementComponent.DisableMovement` (`Character.CharacterMovement` (`GameplayStatics.GetPlayerCharacter` 0))))))

(event `OnSeedPlanted`
  (params (ItemInfos :type "/Game/LS_Template/Blueprints/Systems/Structures/Items/S_ItemInfo Structure"))
  ;[1 1 1] On seed planted, add the item infos in the GardeningPlots map in LST_Instance, sets the plant mesh, updates the plot and the widget
  (`BlueprintMapLibrary.Map_Add` (`/Game/LS_Template/Blueprints/Systems/Core/LS_Instance.GardeningPlots` (`/Game/LS_Template/Blueprints/Systems/Core/BPL_Functions.Get_LST_Instance`)) (`self.PlotIndex`) (`self.ProcessIncomingItemInfo` ItemInfos))
  (`StaticMeshComponent.SetStaticMesh` (`self.SM_PlantMesh`) (`.PlantMesh_10_4DE856D64CF4D381BC45BC8CA68FB0C7` (break `/Game/LS_Template/Blueprints/Systems/Structures/Gardening/S_GardenDetails` (`.GardeningDetails_96_050839D542312D15C483939103ED3120` (break `/Game/LS_Template/Blueprints/Systems/Structures/Items/S_ItemInfo` (`BlueprintMapLibrary.Map_Find` (`/Game/LS_Template/Blueprints/Systems/Core/LS_Instance.GardeningPlots` (`/Game/LS_Template/Blueprints/Systems/Core/BPL_Functions.Get_LST_Instance`)) (`self.PlotIndex`)))))))
  (`self.UpdateGardenPlot`)
  (`/Game/LS_Template/Blueprints/UI/Gardening/W_GardenMenu.UpdateWidget` (`/Game/LS_Template/Blueprints/Systems/Core/LS_Instance.W_GardenMenu` (`/Game/LS_Template/Blueprints/Systems/Core/BPL_Functions.Get_LST_Instance`))))

(fn `EmptyGardenPlot`
  (bind _w_gardenmenu (`/Game/LS_Template/Blueprints/Systems/Core/LS_Instance.W_GardenMenu` (`/Game/LS_Template/Blueprints/Systems/Core/BPL_Functions.Get_LST_Instance`)))
  (`BlueprintMapLibrary.Map_Remove` (`/Game/LS_Template/Blueprints/Systems/Core/LS_Instance.GardeningPlots` (`/Game/LS_Template/Blueprints/Systems/Core/BPL_Functions.Get_LST_Instance`)) (`self.PlotIndex`))
  (`self.UpdateGardenPlot`)
  (`WidgetSwitcher.SetActiveWidgetIndex` (`/Game/LS_Template/Blueprints/UI/Gardening/W_GardenMenu.GardenSwitcher` _w_gardenmenu) 0)
  (set `/Game/LS_Template/Blueprints/UI/Gardening/W_GardenMenu.CancelBarValue` 0.0 _w_gardenmenu)
  (return))

(fn `ProcessIncomingItemInfo`
  (params (IncomingItemInfo :type "/Game/LS_Template/Blueprints/Systems/Structures/Items/S_ItemInfo Structure (by ref)"))
  (returns (OutItemInfo :type "/Game/LS_Template/Blueprints/Systems/Structures/Items/S_ItemInfo Structure"))
  (bind (_itemrowname _itemname _itemdescription _itemtype _clothestype _itemrarity _itemicon _itemsound _simulatephysics_ _itemmesh _itemprice _itemamount _gaindetails _housingdetails _craftingdetails _gardeningdetails) (break `/Game/LS_Template/Blueprints/Systems/Structures/Items/S_ItemInfo` IncomingItemInfo))
  (bind (_currentday _daynumber _currentmonth _eventname _publicholiday_) (`/Game/LS_Template/Blueprints/Systems/Core/BPL_Functions.GetCurrentDate`))
  (bind (_plantmesh _dateplanted _growthdays _daysbeforeharvest _harvesteditemrowname _harvestedamount) (break `/Game/LS_Template/Blueprints/Systems/Structures/Gardening/S_GardenDetails` _gardeningdetails))
  (return (make `/Game/LS_Template/Blueprints/Systems/Structures/Items/S_ItemInfo` _itemrowname _itemname _itemdescription _itemtype "NewEnumerator0" _itemrarity _itemicon _itemsound _simulatephysics_ _itemmesh _itemprice _itemamount _gaindetails _housingdetails _craftingdetails (make `/Game/LS_Template/Blueprints/Systems/Structures/Gardening/S_GardenDetails` _plantmesh (make `/Game/LS_Template/Blueprints/Systems/Structures/Time/S_Date` _currentday _daynumber _currentmonth _eventname _publicholiday_) _growthdays _growthdays _harvesteditemrowname _harvestedamount))))

(fn `SetOutline?`
  (params (`Outline?` :type Boolean))
  (bind _sm_plantmesh (`self.SM_PlantMesh`))
  (if (`/Game/LS_Template/Blueprints/Systems/Core/LS_Instance.UseMeshOutline?` (`/Game/LS_Template/Blueprints/Systems/Core/BPL_Functions.Get_LST_Instance`))
    (`MaterialInstanceDynamic.SetVectorParameterValue` (`/Game/LS_Template/Blueprints/Interaction/Core/BPC_Interaction.OutlineDynamat` (`/Game/LS_Template/Blueprints/Systems/Core/Game/BP_LS_GameController.BPC_Interaction` (`/Game/LS_Template/Blueprints/Systems/Core/BPL_Functions.Get_LST_Controller`))) "OutlineColor" (struct :`R` 0.147275 :`G` 0.994792 :`B` 0.077031 :`A` 1.0))
    (`/Engine/EditorBlueprintResources/StandardMacros.IsValid` _sm_plantmesh
      (:`Is Valid`
        (`PrimitiveComponent.SetRenderCustomDepth` _sm_plantmesh `Outline?`)
        (return)))
    (else
      (return))))

(fn `UpdateGardenPlot`
  (bind _interactionactor (`self.InteractionActor`))
  (bind (_plantmesh _dateplanted _growthdays _daysbeforeharvest _harvesteditemrowname _harvestedamount) (break `/Game/LS_Template/Blueprints/Systems/Structures/Gardening/S_GardenDetails` (`.GardeningDetails_96_050839D542312D15C483939103ED3120` (break `/Game/LS_Template/Blueprints/Systems/Structures/Items/S_ItemInfo` (`BlueprintMapLibrary.Map_Find` (`/Game/LS_Template/Blueprints/Systems/Core/LS_Instance.GardeningPlots` (`/Game/LS_Template/Blueprints/Systems/Core/BPL_Functions.Get_LST_Instance`)) (`self.PlotIndex`))))))
  (bind _returnvalue (`KismetTextLibrary.Conv_IntToText` _harvestedamount))
  (bind _returnvalue_2 (/ 1.0 (+ (`KismetMathLibrary.Conv_IntToDouble` _daysbeforeharvest) 1.0)))
  (`/Engine/EditorBlueprintResources/StandardMacros.IsValid` _plantmesh
    (:`Is Valid`
      (`SceneComponent.SetRelativeScale3D` (`self.SM_PlantMesh`) (`KismetMathLibrary.MakeVector` _returnvalue_2 _returnvalue_2 _returnvalue_2))
      (bind _returnvalue_3 (`|GetDataTableRow` "/Game/LS_Template/Blueprints/Items/DT_Items.DT_Items" _harvesteditemrowname)
        (:`then`
          (bind (_itemrowname _itemname) (break `/Game/LS_Template/Blueprints/Systems/Structures/Items/S_ItemInfo` _returnvalue_3))
          (`/Game/LS_Template/Blueprints/Interaction/Core/BP_InteractionActor.SetWidget` (`self.InteractionActor`) (select `bool` (<= _daysbeforeharvest 0) :`false` (`|FormatText` "{ItemName} x {Amount} \n({Days} days)" _itemname _returnvalue (`KismetTextLibrary.Conv_IntToText` _daysbeforeharvest)) :`true` (`|FormatText` "{ItemName} x {Amount} \n(Harvestable)" _itemname _returnvalue)) false 0 0)
          (return))))
    (:`Is Not Valid`
      (`StaticMeshComponent.SetStaticMesh` (`self.SM_PlantMesh`) null)
      (`/Game/LS_Template/Blueprints/Interaction/Core/BP_InteractionActor.SetWidget` _interactionactor "Empty" false 0 0)
      (`/Game/LS_Template/Blueprints/Interaction/Core/BP_InteractionActor.HidePrompt` _interactionactor true)
      (return))))

(fn `UserConstructionScript`
  (bind _interactionactor (`self.InteractionActor`))
  (bind _asbp_interaction_actor (cast `/Game/LS_Template/Blueprints/Interaction/Core/BP_InteractionActor` (`ChildActorComponent.ChildActor` (`self.ChildActor`))))
  (set `self.InteractionActor` _asbp_interaction_actor)
  (`/Game/LS_Template/Blueprints/Interaction/Core/BP_InteractionActor.HandleInteractionShape` _interactionactor (`self.InteractionShape`) (`self.SphereRadius`) (`self.BoxExtent`) (`self.CapsuleHalfHeight`) (`self.CapsuleRadius`))
  (`self.K2_SetActorRelativeLocation` _interactionactor (`self.InteractionLocation`) false false)
  (`SceneComponent.K2_SetRelativeLocation` (`/Game/LS_Template/Blueprints/Interaction/Core/BP_InteractionActor.Widget` _interactionactor) (`self.PromptLocation`) false false))